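; Interpreter for SLang, a small scripting language, that runs a script string and reports the result through OnExit.
; Run tokenizes characters, parses semicolon-delimited statements, then evaluates the AST from its root.
; Expressions pass through shunting-yard conversion to RPN, then a stack builds literal, identifier, unary and binary node objects under the root.
; Operator arity is inferred during parsing by evaluating the top stack nodes.
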(event `Run`
  ;[1 1 1] Run
  (`self.Tokenize`)
  (`self.Parse Tokens`)
  (`self.Execute AST`))

(event `Parse Next Statement`
  (bind _currenttoken_type (break `/Game/BPSLang/S_SLangToken` (`self.CurrentToken`)))
  ;[1 1 1] Parsing
  (bind _success (`self.NextToken`))
  (if _success
    (if (< (`self.Position`) (`KismetArrayLibrary.Array_Length` (`self.Tokens`))) :!label _label
      (set `self.CurrentToken` (`|GetArrayItem` (`self.Tokens`) (`self.Position`)))
      (if (> (`KismetMathLibrary.And_IntInt` (`self.TokenTypeToBitmask` _currenttoken_type) (`|BitmaskLiteral` 5)) 0)
        (bind _success_2 (`self.ParseExpression`))
        (if _success_2
          (`self.Parse Next Statement`)
          (else
            (`self.OnExit` "Parse Failed" :!label _label_2)))
        (else
          (goto _label_2)))
      (else
        (set `self.ParseOK` true :!label _label_3)
        (`self.ParsingFinished`)))
    (else
      (goto _label_3))))

(event `Parse Tokens`
  ;[1 1 1] Parsing
  (bind _returnvalue (`|GenericCreateObject` "/Game/BPSLang/AST/BP_ASTNode_Root.BP_ASTNode_Root_C" self))
  (set `self.ASTRoot` _returnvalue)
  (set `self.ParseOK` false)
  (set `self.Position` 0)
  (set `self.TokensLen` (`KismetArrayLibrary.Array_Length` (`self.Tokens`)))
  (goto _label))

(event `Continue Tokenize`
  (bind _currentchar (`self.CurrentChar`))
  (bind _position (`self.Position`))
  (bind (_value _returnvalue) (`BlueprintMapLibrary.Map_Find` (`self.Keywords`) (`self.TokenBuilder`)))
  (bind _returnvalue_2 (`KismetStringLibrary.EqualEqual_StrStr` (`self.CurrentChar`) "\""))
  (bind (_value_2 _returnvalue_3) (`BlueprintMapLibrary.Map_Find` (`self.SpecialCharacters`) _currentchar))
  (bind _returnvalue_4 (`KismetMathLibrary.InRange_IntInt` (`KismetStringLibrary.GetCharacterAsNumber` (`self.CurrentChar`)) 48 57))
  (bind _returnvalue_5 (`KismetMathLibrary.InRange_IntInt` (`KismetStringLibrary.GetCharacterAsNumber` (`KismetStringLibrary.ToUpper` (`self.CurrentChar`))) 65 90))
  ;[1 1 1] Tokenize
  (if (< _position (`self.ScriptLen`)) :!label _label_4
    (set `self.TokenBuilder` "")
    (bind _output_get (set `self.CurrentChar` (`|GetArrayItem` (stale `Tokenize` _output_get) _position)))
    (if (or (`KismetStringLibrary.EqualEqual_StrStr` _output_get " ") (`KismetStringLibrary.EqualEqual_StrStr` _output_get " \n ") (`KismetStringLibrary.IsEmpty` _output_get))
      (`self.TokNextChar`)
      (`self.Continue Tokenize`)
      (else
        ;;[1 1 1] Integer Literal
        (if _returnvalue_4
          (while _returnvalue_4
            (set `self.TokenBuilder` (`KismetStringLibrary.Concat_StrStr` (`self.TokenBuilder`) (`self.CurrentChar`)))
            (`self.TokNextChar`))
          (`KismetArrayLibrary.Array_Add` (`self.Tokens`) (make `/Game/BPSLang/S_SLangToken` "NewEnumerator4" (`self.TokenBuilder`)))
          (`self.Continue Tokenize`)
          (else
            ;;[1 1 1] String Literal
            (if _returnvalue_2
              (`self.TokNextChar`)
              (while (not _returnvalue_2)
                (set `self.TokenBuilder` (`KismetStringLibrary.Concat_StrStr` (`self.TokenBuilder`) (`self.CurrentChar`)))
                (`self.TokNextChar` :!label _label_5))
              (`|ExecutionSequence`
                (:`then_0`
                  (goto _label_5))
                (:`then_1`
                  (`KismetArrayLibrary.Array_Add` (`self.Tokens`) (make `/Game/BPSLang/S_SLangToken` "NewEnumerator5" (`self.TokenBuilder`)))
                  (`self.Continue Tokenize`)))
              (else
                ;;[1 1 1] Identifier / Keyword
                (if _returnvalue_5
                  (while _returnvalue_5
                    (set `self.TokenBuilder` (`KismetStringLibrary.Concat_StrStr` (`self.TokenBuilder`) (`self.CurrentChar`)))
                    (`self.TokNextChar`))
                  (`KismetArrayLibrary.Array_Add` (`self.Tokens`) (make `/Game/BPSLang/S_SLangToken` (select `bool` _returnvalue :`false` "NewEnumerator1" :`true` _value) (`self.TokenBuilder`)))
                  (`self.Continue Tokenize`)
                  (else
                    ;;[1 1 1] Spec Char
                    (if _returnvalue_3
                      (`KismetArrayLibrary.Array_Add` (`self.Tokens`) (make `/Game/BPSLang/S_SLangToken` _value_2 _currentchar)))
                    (`self.TokNextChar`)
                    (`self.Continue Tokenize`)))))))))
    (else
      (`self.TokenizeFinished`))))

(event `Tokenize`
  (bind _returnvalue (`KismetStringLibrary.GetCharacterArrayFromString` (`self.Script`)))
  ;[1 1 1] Tokenize
  ;;[1 1 1] Break down the script to characters and save Len
  (`KismetArrayLibrary.Array_Clear` (`self.Tokens`))
  (bind _output_get (set `self.ScriptCharacters` _returnvalue))
  (set `self.ScriptLen` (`KismetArrayLibrary.Array_Length` _returnvalue))
  (goto _label_4))

(event `Execute AST`
  ;[1 1 1] Execution
  (`BlueprintMapLibrary.Map_Clear` (`self.ProgramMemory`))
  (if (`self.ParseOK`)
    (bind (_token _success) (`/Game/BPSLang/AST/BP_ASTNode.Evaluate` (`self.ASTRoot`) "Program"))
    (if _success
      (`self.OnExit` (`.Value_5_0A1308534E7CCF79AC582795E90C5C32` (break `/Game/BPSLang/S_SLangToken` _token)))
      (else
        (`self.OnExit` "Program Failed")))))

(fn `BitmaskToTokenType`
  (params (Bitmask :type Integer))
  (returns (Type :type "/Game/BPSLang/E_SLangTokenTypes Enum"))
  (return (cast `/Game/BPSLang/E_SLangTokenTypes` (`KismetMathLibrary.Conv_IntToByte` (`KismetMathLibrary.FTrunc` (`KismetMathLibrary.Log` (`KismetMathLibrary.Conv_IntToDouble` Bitmask) 2.0))))))

(fn `ExpectToken`
  (params (`Token Types` :type Integer) (SkipNextToken :type Boolean))
  (returns (Success :type Boolean) (Type :type "/Game/BPSLang/E_SLangTokenTypes Enum") (End :type Boolean))
  (bind _currenttoken_type (break `/Game/BPSLang/S_SLangToken` (`self.CurrentToken`)))
  (bind _returnvalue (> (`KismetMathLibrary.And_IntInt` `Token Types` (`self.TokenTypeToBitmask` _currenttoken_type)) 0))
  (if SkipNextToken
    (return _returnvalue _currenttoken_type false)
    (else
      (bind _success (`self.NextToken`))
      (return _returnvalue _currenttoken_type (not _success)))))

(fn `GetTokenAssociativity`
  (params (Token :type "/Game/BPSLang/S_SLangToken Structure"))
  (returns (`Associativity Right` :type Boolean))
  (return (select `/Game/BPSLang/E_SLangTokenTypes` (`.Type_2_326348144587A733F961328DC9D9CF2D` (break `/Game/BPSLang/S_SLangToken` Token)) :`NewEnumerator2` true :`NewEnumerator17` true)))

(fn `GetTokenPrecedence`
  (params (Token :type "/Game/BPSLang/S_SLangToken Structure"))
  (returns (PrecedenceLevel :type Integer))
  (return (select `/Game/BPSLang/E_SLangTokenTypes` (`.Type_2_326348144587A733F961328DC9D9CF2D` (break `/Game/BPSLang/S_SLangToken` Token)) :`NewEnumerator2` 1 :`NewEnumerator12` 3 :`NewEnumerator13` 3 :`NewEnumerator15` 4 :`NewEnumerator16` 4 :`NewEnumerator17` 6 :`NewEnumerator18` 5 :`NewEnumerator19` 2)))

(fn `IsTokenGeneralTypeAnOperand`
  (params (Type :type "/Game/BPSLang/E_TokenGeneralType Enum" :default "NewEnumerator0"))
  (returns (Yes :type Boolean))
  (return (select `/Game/BPSLang/E_TokenGeneralType` Type :`NewEnumerator4` true :`NewEnumerator1` true :`NewEnumerator2` true)))

(fn `MakeASTExpressionFromRPN`
  (params (RPN :type "Array of /Game/BPSLang/S_RPNToken Structure"))
  (returns (Node :type "/Game/BPSLang/AST/BP_ASTNode Object Reference") (Success :type Boolean))
  (locals (`AST Stack` :type "Array of /Game/BPSLang/AST/BP_ASTNode Object Reference") (CurrentRPNToken :type "/Game/BPSLang/S_RPNToken Structure"))
  (bind _ast_stack (`local.AST Stack`))
  (bind (_currentrpntoken_basetoken _currentrpntoken_precedence _currentrpntoken_rightassociative _currentrpntoken_rpntype _currentrpntoken_tokengeneraltype) (break `/Game/BPSLang/S_RPNToken` (`local.CurrentRPNToken`)))
  (bind _ast_stack_2 (`local.AST Stack`))
  (bind _ast_stack_3 (`local.AST Stack`))
  (bind ((`BaseToken_2_10A8C49740649CD978B9799AED864FEA` _basetoken)) (break `/Game/BPSLang/S_RPNToken` (`local.CurrentRPNToken`)))
  (bind _returnvalue (`KismetArrayLibrary.Array_LastIndex` _ast_stack))
  (bind _returnvalue_2 (`KismetArrayLibrary.Array_IsNotEmpty` _ast_stack_3))
  (bind _type (break `/Game/BPSLang/S_SLangToken` (`.BaseToken_2_10A8C49740649CD978B9799AED864FEA` (break `/Game/BPSLang/S_RPNToken` (`local.CurrentRPNToken`)))))
  (bind _returnvalue_3 (`KismetArrayLibrary.Array_IsValidIndex` _ast_stack _returnvalue))
  (bind _output (`|GetArrayItem` _ast_stack _returnvalue))
  (bind _returnvalue_4 (- _returnvalue 1))
  (bind _returnvalue_5 (`KismetArrayLibrary.Array_IsValidIndex` _ast_stack _returnvalue_4))
  (for _array_element RPN
    (bind _output_get (set `local.CurrentRPNToken` _array_element))
    (`|ExecutionSequence`
      (:`then_0`
        (switch `/Game/BPSLang/E_TokenGeneralType` _currentrpntoken_tokengeneraltype
          (:`NewEnumerator0`
            (bind _ast_node (`self.Pop AST Expr Stack` (`local.AST Stack`)))
            (bind _returnvalue_6 (`|GenericCreateObject` "/Game/BPSLang/AST/Expressions/BP_ASTNode_Unary.BP_ASTNode_Unary_C" _ast_node "NewEnumerator4" self))
            (`KismetArrayLibrary.Array_Add` (`local.AST Stack`) _returnvalue_6))
          (:`NewEnumerator4`
            (bind _returnvalue_7 (`|GenericCreateObject` "/Game/BPSLang/AST/Expressions/BP_ASTNode_Literal.BP_ASTNode_Literal_C" _basetoken self))
            (`KismetArrayLibrary.Array_Add` (`local.AST Stack`) _returnvalue_7))
          (:`NewEnumerator1`
            (bind _returnvalue_8 (`|GenericCreateObject` "/Game/BPSLang/AST/Expressions/BP_ASTNode_Identifier.BP_ASTNode_Identifier_C" (`.Value_5_0A1308534E7CCF79AC582795E90C5C32` (break `/Game/BPSLang/S_SLangToken` _basetoken)) self))
            (`KismetArrayLibrary.Array_Add` (`local.AST Stack`) _returnvalue_8))
          (:`NewEnumerator3`
            (`|ExecutionSequence`
              (:`then_0`
                (if (and _returnvalue_3 _returnvalue_5)
                  (bind (_token _success) (`/Game/BPSLang/AST/BP_ASTNode.Evaluate` _output "AST"))
                  (if _success
                    (bind (_token_2 _success_2) (`/Game/BPSLang/AST/BP_ASTNode.Evaluate` (`|GetArrayItem` _ast_stack _returnvalue_4) "AST"))
                    (if _success_2
                      (bind _yes (`self.IsTokenGeneralTypeAnOperand` (`self.Token To General Type` _token)))
                      (setmembers `/Game/BPSLang/S_RPNToken` :`StructRef` (`local.CurrentRPNToken`) :`RPNType` (select `bool` (and (`self.IsTokenGeneralTypeAnOperand` (`self.Token To General Type` _token_2)) _yes) :`false` (select `bool` _yes :`false` "NewEnumerator0" :`true` "NewEnumerator1" :!type "/Game/BPSLang/E_SlangRPNOpType Enum") :`true` "NewEnumerator2"))
                      (else
                        (return null false)))
                    (else
                      (return null false)))
                  (elif (or _returnvalue_3 _returnvalue_5)
                    (bind (_token_3 _success_3) (`/Game/BPSLang/AST/BP_ASTNode.Evaluate` _output "AST"))
                    (if _success_3
                      (setmembers `/Game/BPSLang/S_RPNToken` :`StructRef` (`local.CurrentRPNToken`) :`RPNType` (select `bool` (`self.IsTokenGeneralTypeAnOperand` (`self.Token To General Type` _token_3)) :`false` "NewEnumerator0" :`true` "NewEnumerator1" :!type "/Game/BPSLang/E_SlangRPNOpType Enum"))
                      (else
                        (return null false)))
                    (else
                      (`KismetSystemLibrary.PrintString` null (`KismetStringLibrary.Concat_StrStr` "Can't operate on no operands, btw AST stack len: " (`KismetStringLibrary.Conv_IntToString` (`KismetArrayLibrary.Array_Length` (`local.AST Stack`)))))
                      (return null false)))))
              (:`then_1`
                (switch `/Game/BPSLang/E_SlangRPNOpType` (`.RPNType_11_807B6652464282ED726FFEB6054DFF8B` (break `/Game/BPSLang/S_RPNToken` (`local.CurrentRPNToken`)))
                  (:`NewEnumerator0`
                    (`KismetSystemLibrary.PrintString` null "Operator Was Nonary!!!")
                    (return null false))
                  (:`NewEnumerator1`
                    (bind _ast_node_2 (`self.Pop AST Expr Stack` (`local.AST Stack`)))
                    (bind _returnvalue_9 (`|GenericCreateObject` "/Game/BPSLang/AST/Expressions/BP_ASTNode_Unary.BP_ASTNode_Unary_C" _ast_node_2 (`self.TokenTypeToUnaryOpType` _type) self))
                    (`KismetArrayLibrary.Array_Add` (`local.AST Stack`) _returnvalue_9))
                  (:`NewEnumerator2`
                    (bind _ast_node_3 (`self.Pop AST Expr Stack` _ast_stack_2))
                    (bind _ast_node_4 (`self.Pop AST Expr Stack` _ast_stack_2))
                    (bind _returnvalue_10 (`|GenericCreateObject` "/Game/BPSLang/AST/Expressions/BP_ASTNode_BinaryOperation.BP_ASTNode_BinaryOperation_C" _ast_node_4 _ast_node_3 (`self.TokenTypeToBinaryOpType` _type) self))
                    (`KismetArrayLibrary.Array_Add` (`local.AST Stack`) _returnvalue_10))))))))))
  (if (not _returnvalue_2)
    (`KismetSystemLibrary.PrintString` null "Making AST Expr Failed"))
  (return (`|GetArrayItem` _ast_stack_3) _returnvalue_2))

(fn `NextToken`
  (returns (Success :type Boolean))
  (bind _tokens (`self.Tokens`))
  (bind _result (`/Engine/EditorBlueprintResources/StandardMacros.IncrementInt` (`self.Position`))
    (:`  `
      (if (`KismetArrayLibrary.Array_IsValidIndex` _tokens _result)
        (set `self.CurrentToken` (`|GetArrayItem` _tokens _result))
        (return true)
        (else
          (return false))))))

(fn `ParseExpression`
  (returns (Success :type Boolean))
  (bind (_rpn _success) (`self.ParseRPN` true))
  (if _success
    (bind (_node _success_2) (`self.MakeASTExpressionFromRPN` _rpn))
    (if _success_2
      (`/Game/BPSLang/AST/BP_ASTNode_Root.AddNode` (`self.ASTRoot`) _node)
      (return true)
      (else
        _)))
  (`KismetSystemLibrary.PrintString` null "Parsing StmntExpr Failed")
  (return false))

(fn `ParseRPN`
  (params (FirstNoNextToken :type Boolean))
  (returns (RPN :type "Array of /Game/BPSLang/S_RPNToken Structure") (Success :type Boolean))
  (locals (Output :type "Array of /Game/BPSLang/S_RPNToken Structure") (Operations :type "Array of /Game/BPSLang/S_RPNToken Structure") (PastFirst :type Boolean) (CurrentRPNToken :type "/Game/BPSLang/S_RPNToken Structure"))
  (bind _currenttoken (`self.CurrentToken`))
  (bind (_currentrpntoken_basetoken _currentrpntoken_precedence _currentrpntoken_rightassociative) (break `/Game/BPSLang/S_RPNToken` (`local.CurrentRPNToken`)))
  (bind _output (`local.Output`))
  (bind _operations (`local.Operations`))
  (bind _operations_2 (`local.Operations`))
  (bind _operations_3 (`local.Operations`))
  (bind _returnvalue (`KismetArrayLibrary.Array_IsNotEmpty` _output))
  (bind _returnvalue_2 (`KismetArrayLibrary.Array_LastIndex` _operations_2))
  (bind _returnvalue_3 (`KismetArrayLibrary.Array_LastIndex` _operations))
  (bind (_output_basetoken _output_precedence) (break `/Game/BPSLang/S_RPNToken` (`|GetArrayItem` _operations_3 (`KismetArrayLibrary.Array_LastIndex` _operations_3))))
  (if (not (select `bool` (`local.PastFirst`) :`false` FirstNoNextToken)) :!label _label
    (bind _success (`self.NextToken`)))
  (if (not (select `bool` (`local.PastFirst`) :`true` (not _success)))
    (set `local.PastFirst` true)
    (set `local.CurrentRPNToken` (make `/Game/BPSLang/S_RPNToken` _currenttoken (`self.GetTokenPrecedence` _currenttoken) (`self.GetTokenAssociativity` _currenttoken) "NewEnumerator0" "NewEnumerator4"))
    (switch `/Game/BPSLang/E_SLangTokenTypes` (`.Type_2_326348144587A733F961328DC9D9CF2D` (break `/Game/BPSLang/S_SLangToken` _currenttoken))
      (:`NewEnumerator0`
        (setmembers `/Game/BPSLang/S_RPNToken` :`StructRef` (`local.CurrentRPNToken`) :`TokenGeneralType` "NewEnumerator0")
        (if (`KismetArrayLibrary.Array_IsEmpty` (`local.Operations`)) :!label _label_2
          _
          (elif (select `bool` _currentrpntoken_rightassociative :`false` (>= _output_precedence _currentrpntoken_precedence) :`true` (> _output_precedence _currentrpntoken_precedence))
            (`KismetArrayLibrary.Array_Add` (`local.Output`) (`|GetArrayItem` _operations_2 _returnvalue_2))
            (`KismetArrayLibrary.Array_Remove` _operations_2 _returnvalue_2)))
        (`KismetArrayLibrary.Array_Add` (`local.Operations`) (`local.CurrentRPNToken`))
        (goto _label))
      (:`NewEnumerator14`
        (setmembers `/Game/BPSLang/S_RPNToken` :`StructRef` (`local.CurrentRPNToken`) :`TokenGeneralType` "NewEnumerator4" :!label _label_3)
        (`KismetArrayLibrary.Array_Add` (`local.Output`) (`local.CurrentRPNToken`) :!label _label_4)
        (goto _label))
      (:`NewEnumerator1`
        (setmembers `/Game/BPSLang/S_RPNToken` :`StructRef` (`local.CurrentRPNToken`) :`TokenGeneralType` "NewEnumerator1")
        (goto _label_4))
      (:`NewEnumerator2`
        (setmembers `/Game/BPSLang/S_RPNToken` :`StructRef` (`local.CurrentRPNToken`) :`TokenGeneralType` "NewEnumerator3" :!label _label_5)
        (goto _label_2))
      (:`NewEnumerator4`
        (goto _label_3))
      (:`NewEnumerator20`
        (goto _label_3))
      (:`NewEnumerator5`
        (goto _label_3))
      (:`NewEnumerator6`
        (`KismetArrayLibrary.Array_Add` (`local.Operations`) (`local.CurrentRPNToken`))
        (goto _label))
      (:`NewEnumerator7`
        (while (and (not (`|EnumEquality` (`.Type_2_326348144587A733F961328DC9D9CF2D` (break `/Game/BPSLang/S_SLangToken` _output_basetoken)) "NewEnumerator6")) (`KismetArrayLibrary.Array_IsNotEmpty` (`local.Operations`)))
          (`KismetArrayLibrary.Array_Add` (`local.Output`) (`|GetArrayItem` _operations _returnvalue_3))
          (`KismetArrayLibrary.Array_Remove` _operations _returnvalue_3))
        (if (`KismetArrayLibrary.Array_IsValidIndex` _operations _returnvalue_3)
          (`KismetArrayLibrary.Array_Remove` _operations _returnvalue_3)
          (goto _label)
          (else
            (goto _label))))
      (:`NewEnumerator10`
        _)
      (:`NewEnumerator12`
        (goto _label_5))
      (:`NewEnumerator13`
        (goto _label_5))
      (:`NewEnumerator15`
        (goto _label_5))
      (:`NewEnumerator16`
        (goto _label_5))
      (:`NewEnumerator17`
        (goto _label_5))
      (:`NewEnumerator18`
        (goto _label_5))
      (:`NewEnumerator19`
        (goto _label_5))))
  (bind (_arrayindex _arrayelement) (`/Engine/EditorBlueprintResources/StandardMacros.ReverseForEachLoop` (`local.Operations`))
    (:`LoopBody`
      (`KismetArrayLibrary.Array_Add` (`local.Output`) _arrayelement))
    (:`Completed`
      (if (not _returnvalue)
        (`KismetSystemLibrary.PrintString` null "Paring RPN Failed"))
      (return _output _returnvalue))))

(fn `Pop AST Expr Stack`
  (params (`AST Stack` :type "Array of /Game/BPSLang/AST/BP_ASTNode Object Reference"))
  (returns (`AST Node` :type "/Game/BPSLang/AST/BP_ASTNode Object Reference"))
  (locals (ASTNodeTMP :type "/Game/BPSLang/AST/BP_ASTNode Object Reference"))
  (bind _returnvalue (`KismetArrayLibrary.Array_LastIndex` `AST Stack`))
  (set `local.ASTNodeTMP` (`|GetArrayItem` `AST Stack` _returnvalue))
  (`KismetArrayLibrary.Array_Remove` `AST Stack` _returnvalue)
  (return (`local.ASTNodeTMP`)))

(fn `Token To General Type`
  (params (`Toke Type` :type "/Game/BPSLang/S_SLangToken Structure"))
  (returns (`General Type` :type "/Game/BPSLang/E_TokenGeneralType Enum"))
  (return (select `/Game/BPSLang/E_SLangTokenTypes` (`.Type_2_326348144587A733F961328DC9D9CF2D` (break `/Game/BPSLang/S_SLangToken` `Toke Type`)) :`NewEnumerator0` "NewEnumerator0" :`NewEnumerator14` "NewEnumerator4" :`NewEnumerator1` "NewEnumerator1" :`NewEnumerator2` "NewEnumerator3" :`NewEnumerator4` "NewEnumerator4" :`NewEnumerator20` "NewEnumerator0" :`NewEnumerator5` "NewEnumerator4" :`NewEnumerator6` "NewEnumerator0" :`NewEnumerator7` "NewEnumerator0" :`NewEnumerator10` "NewEnumerator0" :`NewEnumerator12` "NewEnumerator3" :`NewEnumerator13` "NewEnumerator3" :`NewEnumerator15` "NewEnumerator3" :`NewEnumerator16` "NewEnumerator3" :`NewEnumerator17` "NewEnumerator3" :`NewEnumerator18` "NewEnumerator3" :`NewEnumerator19` "NewEnumerator3" :!type "/Game/BPSLang/E_TokenGeneralType Enum")))

(fn `TokenTypeToBinaryOpType`
  (params (`Token Type` :type "/Game/BPSLang/E_SLangTokenTypes Enum" :default "NewEnumerator0"))
  (returns (`Binary Type` :type "/Game/BPSLang/AST/Expressions/E_BinaryOperationType Enum"))
  (return (select `/Game/BPSLang/E_SLangTokenTypes` `Token Type` :`NewEnumerator0` "NewEnumerator0" :`NewEnumerator14` "NewEnumerator0" :`NewEnumerator1` "NewEnumerator0" :`NewEnumerator2` "NewEnumerator4" :`NewEnumerator4` "NewEnumerator0" :`NewEnumerator20` "NewEnumerator0" :`NewEnumerator5` "NewEnumerator0" :`NewEnumerator6` "NewEnumerator0" :`NewEnumerator7` "NewEnumerator0" :`NewEnumerator10` "NewEnumerator0" :`NewEnumerator12` "NewEnumerator0" :`NewEnumerator13` "NewEnumerator1" :`NewEnumerator15` "NewEnumerator2" :`NewEnumerator16` "NewEnumerator3" :`NewEnumerator17` "NewEnumerator5" :`NewEnumerator18` "NewEnumerator0" :`NewEnumerator19` "NewEnumerator6" :!type "/Game/BPSLang/AST/Expressions/E_BinaryOperationType Enum")))

(fn `TokenTypeToBitmask`
  (params (Type :type "/Game/BPSLang/E_SLangTokenTypes Enum" :default "NewEnumerator0"))
  (returns (Bitmask :type Integer))
  (return (`|BitmaskLiteral` (`KismetMathLibrary.FTrunc` (`KismetMathLibrary.MultiplyMultiply_FloatFloat` 2.0 (`KismetMathLibrary.Conv_IntToDouble` (`KismetMathLibrary.Conv_ByteToInt` Type)))))))

(fn `TokenTypeToUnaryOpType`
  (params (`Token Type` :type "/Game/BPSLang/E_SLangTokenTypes Enum" :default "NewEnumerator0"))
  (returns (`Unary Type` :type "/Game/BPSLang/AST/Expressions/E_UnaryOperationType Enum"))
  (return (select `/Game/BPSLang/E_SLangTokenTypes` `Token Type` :`NewEnumerator0` "NewEnumerator0" :`NewEnumerator14` "NewEnumerator0" :`NewEnumerator1` "NewEnumerator0" :`NewEnumerator2` "NewEnumerator0" :`NewEnumerator4` "NewEnumerator0" :`NewEnumerator20` "NewEnumerator0" :`NewEnumerator5` "NewEnumerator0" :`NewEnumerator6` "NewEnumerator0" :`NewEnumerator7` "NewEnumerator0" :`NewEnumerator10` "NewEnumerator0" :`NewEnumerator12` "NewEnumerator0" :`NewEnumerator13` "NewEnumerator0" :`NewEnumerator15` "NewEnumerator0" :`NewEnumerator16` "NewEnumerator0" :`NewEnumerator17` "NewEnumerator0" :`NewEnumerator18` "NewEnumerator1" :`NewEnumerator19` "NewEnumerator0" :!type "/Game/BPSLang/AST/Expressions/E_UnaryOperationType Enum")))

(fn `TokNextChar`
  (bind _scriptcharacters (`self.ScriptCharacters`))
  (bind _result (`/Engine/EditorBlueprintResources/StandardMacros.IncrementInt` (`self.Position`))
    (:`  `
      (if (`KismetArrayLibrary.Array_IsValidIndex` _scriptcharacters _result)
        (set `self.CurrentChar` (`|GetArrayItem` _scriptcharacters _result))))))