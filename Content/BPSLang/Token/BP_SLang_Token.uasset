(fn `AsIdentifier`
  (returns (Value :type String) (Type :type String))
  (return (`self.Value`) (`self.Type`)))

(fn `AsKeyword`
  (returns (Value :type String))
  (return (`self.Value`)))

(fn `AsLiteral`
  (returns (Value :type String) (Type :type String))
  (return (`self.Value`) (`self.Type`)))

(fn `AsOperator`
  (returns (Value :type String) (Precedence :type Integer) (Association :type "/Game/BPSLang/E_TokenAssociation Enum") (Operations :type "Array of /Game/BPSLang/E_TokenOperation Enum"))
  (return (`self.Value`) (`self.Precedence`) (`self.Association`) (`self.PossibleOperations`)))

(fn `AsType`
  (returns (Value :type String))
  (return (`self.Value`)))

(fn `GetOperativeness`
  (returns (ReturnValue :type "/Game/BPSLang/E_TokenOperativeness Enum"))
  (return (select `/Game/BPSLang/E_TokenDomain` (`self.Domain`) :`NewEnumerator0` "NewEnumerator1" :`NewEnumerator4` "NewEnumerator0" :`NewEnumerator1` "NewEnumerator0" :`NewEnumerator3` "NewEnumerator1" :`NewEnumerator5` "NewEnumerator2" :!type "/Game/BPSLang/E_TokenOperativeness Enum")))

(fn `MakeIdentifier`
  (params (Value :type String) (Type :type String))
  (set `self.Value` Value)
  (set `self.Type` Type)
  (set `self.Domain` "NewEnumerator1"))

(fn `MakeKeyword`
  (params (Value :type String))
  (set `self.Value` Value)
  (set `self.Domain` "NewEnumerator0"))

(fn `MakeLiteral`
  (params (Value :type String) (Type :type String))
  (set `self.Value` Value)
  (set `self.Type` Type)
  (set `self.Domain` "NewEnumerator4"))

(fn `MakeOperator`
  (params (Value :type String))
  (returns (Success :type Boolean))
  (locals (OperatorsDatabase :type "/Game/BPSLang/BP_SLang_OperatorsDatabase Object Reference" :default "/Game/BPSLang/BP_SLang_OperatorsDatabase.BP_SLang_OperatorsDatabase_C'/Game/BPSLang/DA_SLang_OperatorsDatabase.DA_SLang_OperatorsDatabase'") (DoubleOperatorsDatabase :type "/Game/BPSLang/BP_SLang_OperatorsDatabase Object Reference" :default "/Game/BPSLang/BP_SLang_OperatorsDatabase.BP_SLang_OperatorsDatabase_C'/Game/BPSLang/DA_SLang_DoubleOperatorsDatabase.DA_SLang_DoubleOperatorsDatabase'") (OperatorDescriptor :type "/Game/BPSLang/S_SLang_OperatorDescriptor Structure"))
  (bind (_operatordescriptor_precedence _operatordescriptor_association _operatordescriptor_operations) (break `/Game/BPSLang/S_SLang_OperatorDescriptor` (`local.OperatorDescriptor`)))
  (bind _output_get (set `self.Value` Value))
  (set `self.Domain` "NewEnumerator3")
  (bind (_value _returnvalue) (`BlueprintMapLibrary.Map_Find` (`/Game/BPSLang/BP_SLang_OperatorsDatabase.Database` (`local.OperatorsDatabase`)) _output_get))
  (if _returnvalue
    (set `local.OperatorDescriptor` _value)
    (else
      (bind (_value_2 _returnvalue_2) (`BlueprintMapLibrary.Map_Find` (`/Game/BPSLang/BP_SLang_OperatorsDatabase.Database` (`local.DoubleOperatorsDatabase`)) _output_get))
      (if _returnvalue_2
        (set `local.OperatorDescriptor` _value_2)
        (else
          (`KismetSystemLibrary.PrintString` null "Operator Not Found")
          (return false)))))
  (set `self.Precedence` _operatordescriptor_precedence)
  (set `self.Association` _operatordescriptor_association)
  (set `self.PossibleOperations` _operatordescriptor_operations)
  (return true))

(fn `MakeType`
  (params (Value :type String))
  (set `self.Value` Value)
  (set `self.Domain` "NewEnumerator5"))