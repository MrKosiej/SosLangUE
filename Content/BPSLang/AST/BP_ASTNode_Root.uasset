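; Root node of the BPSLang abstract syntax tree, holding the top-level expressions and evaluating them as a sequence.
; AddNode appends child nodes to the Expressions array, which Evaluate walks in order, passing "Root" as each child's origin.
; Evaluation stops with failure at the first unsuccessful expression; otherwise it succeeds and returns the token from the last one evaluated.
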(fn `AddNode`
  (params (Node :type "/Game/BPSLang/AST/BP_ASTNode Object Reference"))
  (`KismetArrayLibrary.Array_Add` (`self.Expressions`) Node))

(fn `Evaluate`
  (params (Origin :type String))
  (returns (Token :type "/Game/BPSLang/S_SLangToken Structure") (Success :type Boolean))
  (locals (EvaluationToken :type "/Game/BPSLang/S_SLangToken Structure"))
  (bind _expressions (`self.Expressions`))
  (set `self.ExecutionIndex` 0)
  (if (< (`self.ExecutionIndex`) (`KismetArrayLibrary.Array_Length` _expressions)) :!label _label
    (bind (_token _success) (`self.Evaluate` (`|GetArrayItem` _expressions (`self.ExecutionIndex`)) "Root"))
    (set `local.EvaluationToken` _token)
    (if _success
      (`/Engine/EditorBlueprintResources/StandardMacros.IncrementInt` (`self.ExecutionIndex`)
        (:`  `
          (goto _label)))
      (else
        (return (struct) false)))
    (else
      (return (`local.EvaluationToken`) true))))