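; AST program node for BPSLang, a scripting language built in Blueprint, that runs a script as a callable with typed parameters.
; Evaluate checks argument count and types, storing each argument node in Memory under its parameter name.
; When Parse is set, it lexes and parses Script, passing itself to the parser, before running Expressions.
; Expressions evaluate in order, failing on error, stopping on Return and yielding the last token.
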(fn `AddNode`
  (params (Node :type "/Game/BPSLang/AST/BP_ASTNode Object Reference"))
  (`KismetArrayLibrary.Array_Add` (`self.Expressions`) Node))

(fn `Evaluate`
  (params (Origin :type String))
  (returns (Token :type "/Game/BPSLang/Token/BP_SLang_Token Object Reference") (Success :type Boolean))
  (locals (EvaluationToken :type "/Game/BPSLang/Token/BP_SLang_Token Object Reference"))
  (`KismetSystemLibrary.PrintString` null (`KismetStringLibrary.Concat_StrStr` "Running Program of Origin: " Origin " with " (`KismetStringLibrary.Conv_IntToString` (`KismetArrayLibrary.Array_Length` (`self.Arguments`))) " args") false)
  ;[1 1 1] Match arguments with parameters
  (if (== (`KismetArrayLibrary.Array_Length` (`self.Arguments`)) (`KismetArrayLibrary.Array_Length` (`self.ParamTypes`)))
    (for (_array_element _array_index) (`self.Arguments`)
      (bind (_token _success) (`self.Evaluate` _array_element (`self.ProgramName`)))
      (if _success
        (if (`KismetStringLibrary.EqualEqual_StrStr` (`/Game/BPSLang/Token/BP_SLang_Token.Type` _token) (`|GetArrayItem` (`self.ParamTypes`) _array_index))
          (`BlueprintMapLibrary.Map_Add` (`self.Memory`) (`|GetArrayItem` (`self.ParamNames`) _array_index) _array_element)
          (else
            (`KismetSystemLibrary.PrintString` null "Argument type does not match parameter type" false)
            (return null false)))
        (else
          (`KismetSystemLibrary.PrintString` null "Argument failed to evaluate" false)
          (return null false))))
    ;[1 1 1] Parsing
    (if (`self.Parse`)
      (bind _returnvalue (`|GenericCreateObject` "/Game/BPSLang/BP_SLang_Lexer.BP_SLang_Lexer_C"))
      (bind (_success_2 _tokens) (`/Game/BPSLang/BP_SLang_Lexer.Tokenize` _returnvalue (`self.Script`)))
      (if _success_2
        (bind _returnvalue_2 (`|GenericCreateObject` "/Game/BPSLang/BP_SLang_Parser.BP_SLang_Parser_C" self _tokens))
        (bind _success_3 (`/Game/BPSLang/BP_SLang_Parser.Parse` _returnvalue_2))
        (if _success_3
          _
          (else
            (`KismetSystemLibrary.PrintString` null "Parsing Failed" false)
            (return null false)))
        (else
          (`KismetSystemLibrary.PrintString` null "Lexing Failed" false)
          (return null false))))
    ;[1 1 1] Running expressions
    (for (_array_element_2 _array_index_2) (`self.Expressions`)
      (bind (_token_2 _success_4) (`self.Evaluate` _array_element_2 (`self.ProgramName`)))
      (bind _output_get (set `local.EvaluationToken` _token_2))
      (`/Engine/EditorBlueprintResources/StandardMacros.IsValid` _output_get
        (:`Is Valid`
          (if _success_4
            (switch `/Game/BPSLang/E_FlowControlType` (`/Game/BPSLang/Token/BP_SLang_Token.Flow Control Type` _output_get)
              (:`NewEnumerator1`
                (`KismetSystemLibrary.PrintString` null "Flow Control Return")
                (break)))
            (else
              (`KismetSystemLibrary.PrintString` null (`KismetStringLibrary.Concat_StrStr` "Failed to evaluate Expression: " (`KismetStringLibrary.Conv_IntToString` _array_index_2)) false)
              (return null false))))
        (:`Is Not Valid`
          (`KismetSystemLibrary.PrintString` null "Eval Token invalid" false)
          (return null false))))
    (return (`local.EvaluationToken`) true)
    (else
      (`KismetSystemLibrary.PrintString` null "Args len does not match param len" false)
      (return null false))))