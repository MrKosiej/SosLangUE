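; AST node for the BPSLang scripting language that declares a program and stores it in the memory of its enclosing program context.
; Execute copies the body expressions unevaluated, then runs the name, return type and parameter child nodes in sequence through bind/unbind OnExecuted callbacks.
; An index counter steps through parameters, recording names and types.
; It finishes with a name/return-type token, or reports failure when any child fails.
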(event `self.Execute`
  (params (Origin :type String))
  (bind _programname (`self.ProgramName`))
  (set `self.ParamLoopIndex` 0)
  (set `self.ProgramContext` (`/Game/BPSLang/AST/BP_ASTNode.ProgramContext` (`self.DeclaredProgram`)))
  (set `/Game/BPSLang/AST/BP_ASTNode_Program.Expressions` (`/Game/BPSLang/AST/BP_ASTNode_ExpressionsWrapper.Expressions` (`self.Body`)) (`self.DeclaredProgram`))
  ;[1 1 1] Prog Name
  (add `self.OnExecuted` _programname (delegate `OnProgNameExecuted_Event`))
  (`self.Execute` _programname "Program Decl Name"))

(event `OnProgNameExecuted_Event` :!signature `self.OnExecuted`
  (params (Token :type "/Game/BPSLang/Token/BP_SLang_Token Object Reference") (Success :type Boolean))
  (bind _returntype (`self.ReturnType`))
  ;[1 1 1] Prog Name
  (remove `self.OnExecuted` (`self.ProgramName`) (delegate `OnProgNameExecuted_Event`))
  (`/Engine/EditorBlueprintResources/StandardMacros.IsValid` Token
    (:`Is Valid`
      (if Success
        (set `/Game/BPSLang/AST/BP_ASTNode_Program.ProgramName` (`/Game/BPSLang/Token/BP_SLang_Token.Value` Token) (`self.DeclaredProgram`))
        ;[1 1 1] Prog Return Type
        (add `self.OnExecuted` _returntype (delegate `OnReturnTypeExecuted_Event`))
        (`self.Execute` _returntype "Program Decl Return Type")
        (else
          (`KismetSystemLibrary.PrintString` null "Prog Name Node invalid or unsuccessful" :!label _label)
          (`self.OnExecuted` null))))
    (:`Is Not Valid`
      (goto _label))))

(event `ContinueExecutingParams`
  (bind _programcontext (`self.ProgramContext`))
  (bind _parameters (`self.Parameters`))
  (bind _paramloopindex (`self.ParamLoopIndex`))
  (bind _declaredprogram (`self.DeclaredProgram`))
  (bind _output (`|GetArrayItem` _parameters _paramloopindex))
  (bind _programname (`/Game/BPSLang/AST/BP_ASTNode_Program.ProgramName` _declaredprogram))
  ;[1 1 1] Params
  (if (`KismetArrayLibrary.Array_IsValidIndex` _parameters _paramloopindex) :!label _label_2
    (add `self.OnExecuted` _output (delegate `OnParamNodeExecuted_Event`))
    (`self.Execute` _output "Prog Decl Param")
    (else
      (bind _returnvalue (`|GenericCreateObject` "/Game/BPSLang/Token/BP_SLang_Token.BP_SLang_Token_C"))
      (`/Game/BPSLang/Token/BP_SLang_Token.MakeStandardToken` _returnvalue _programname (`/Game/BPSLang/AST/BP_ASTNode_Program.Return Type` _declaredprogram) "NewEnumerator1")
      (`BlueprintMapLibrary.Map_Add` (`/Game/BPSLang/AST/BP_ASTNode_Program.Memory` _programcontext) _programname (`self.DeclaredProgram`))
      (`KismetSystemLibrary.PrintString` null (`KismetStringLibrary.Concat_StrStr` "Saving Program: " _programname " To the memory of " (`/Game/BPSLang/AST/BP_ASTNode_Program.ProgramName` _programcontext)))
      (`self.OnExecuted` _returnvalue true))))

(event `OnReturnTypeExecuted_Event` :!signature `self.OnExecuted`
  (params (Token :type "/Game/BPSLang/Token/BP_SLang_Token Object Reference") (Success :type Boolean))
  ;[1 1 1] Prog Return Type
  (remove `self.OnExecuted` (`self.ReturnType`) (delegate `OnReturnTypeExecuted_Event`))
  (`/Engine/EditorBlueprintResources/StandardMacros.IsValid` Token
    (:`Is Valid`
      (if Success
        (set `/Game/BPSLang/AST/BP_ASTNode_Program.Return Type` (`/Game/BPSLang/Token/BP_SLang_Token.Value` Token) (`self.DeclaredProgram`))
        (goto _label_2)
        (else
          _)))
    (:`Is Not Valid`
      _))
  (`KismetSystemLibrary.PrintString` null "Prog Return Type Node invalid or unsuccessful")
  (`self.OnExecuted` null))

(event `OnParamNodeExecuted_Event` :!signature `self.OnExecuted`
  (params (Token :type "/Game/BPSLang/Token/BP_SLang_Token Object Reference") (Success :type Boolean))
  (bind (_value _type) (`/Game/BPSLang/Token/BP_SLang_Token.GetStandardDetails` Token))
  ;[1 1 1] Params
  (remove `self.OnExecuted` (`|GetArrayItem` (`self.Parameters`) (`self.ParamLoopIndex`)) (delegate `OnParamNodeExecuted_Event`))
  (`/Engine/EditorBlueprintResources/StandardMacros.IsValid` Token
    (:`Is Valid`
      (if Success
        (`KismetArrayLibrary.Array_Add` (`/Game/BPSLang/AST/BP_ASTNode_Program.ParamNames` (`self.DeclaredProgram`)) _value)
        (`KismetArrayLibrary.Array_Add` (`/Game/BPSLang/AST/BP_ASTNode_Program.ParamTypes` (`self.DeclaredProgram`)) _type)
        (`/Engine/EditorBlueprintResources/StandardMacros.IncrementInt` (`self.ParamLoopIndex`)
          (:`  `
            (`self.ContinueExecutingParams`)))
        (else
          (`KismetSystemLibrary.PrintString` null "Prog Param Node invalid or unsuccessful" :!label _label_3)
          (`self.OnExecuted` null))))
    (:`Is Not Valid`
      (goto _label_3))))