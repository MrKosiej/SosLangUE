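; AST node for a program call in a Blueprint-built scripting language interpreter.
; It evaluates its identifier node, then searches the name up the chain of parent program contexts' memory.
; The matching program node receives the call's arguments and runs asynchronously through OnExecuted delegates, passing back its result or failure.
; Duplicate shares this path, but on success only prints a message without firing OnExecuted.
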(event `self.Duplicate`
  (bind _identifier (`self.Identifier`))
  ;[1 1 1] Program ID
  (set `self.Duplicating` true)
  (add `self.OnExecuted` _identifier (delegate `OnProgCallIDExec_Event`) :!label _label)
  (`self.Execute` _identifier "Program Call ID" "NewEnumerator0"))

(event `self.Execute`
  (params (Origin :type String) (ReturnType :type "/Game/BPSLang/E_RefVal Enum" :default "NewEnumerator0"))
  ;[1 1 1] Program ID
  (set `self.Duplicating` false)
  (goto _label))

(event `OnProgCallIDExec_Event` :!signature `self.OnExecuted`
  (params (Result :type "/Game/BPSLang/AST/BP_ASTNode Object Reference") (Success :type Boolean))
  (bind _value (`self.GetIdentity` Result))
  ;[1 1 1] Program ID
  (remove `self.OnExecuted` (`self.Identifier`) (delegate `OnProgCallIDExec_Event`))
  (if Success
    (set `self.CurrentProgramContext` (`/Game/BPSLang/AST/BP_ASTNode.ProgramContext` (`self.Identifier`)))
    ;[1 1 1] Find in context Tree
    (bind _currentprogramcontext (`self.CurrentProgramContext`)
      (:`then`
        (bind (_value_2 _returnvalue) (`BlueprintMapLibrary.Map_Find` (`/Game/BPSLang/AST/BP_ASTNode_Program.Memory` _currentprogramcontext) _value))
        (if _returnvalue :!label _label_2
          ;[1 1 1] Passing args and executing
          (bind _asbp_astnode_program (cast `/Game/BPSLang/AST/BP_ASTNode_Program` _value_2)
            (:`then`
              (set `/Game/BPSLang/AST/BP_ASTNode_Program.Arguments` (`self.Arguments`) _asbp_astnode_program)
              (add `self.OnExecuted` _asbp_astnode_program (delegate `OnProgramExecuted_Event`))
              (`self.Execute` _asbp_astnode_program "Program Call" "NewEnumerator1"))
            (:`CastFailed`
              (`KismetSystemLibrary.PrintString` null (`KismetStringLibrary.Concat_StrStr` "Node not a program | " (`KismetSystemLibrary.GetDisplayName` _asbp_astnode_program)) false)
              (`self.OnExecuted` null)))
          (else
            (bind _programcontext (`/Game/BPSLang/AST/BP_ASTNode.ProgramContext` _currentprogramcontext)
              (:`then`
                (set `self.CurrentProgramContext` _programcontext)
                (goto _label_2))
              (:`else`
                (`KismetSystemLibrary.PrintString` null (`KismetStringLibrary.Concat_StrStr` "Did not find ( " _value " ) in program context with name: " (`/Game/BPSLang/AST/BP_ASTNode_Program.ProgramName` _currentprogramcontext)) false :!label _label_3)
                (`self.OnExecuted` null))))))
      (:`else`
        (goto _label_3)))
    (else
      (`KismetSystemLibrary.PrintString` null "Prog Call ID Node invalid or unsuccessful")
      (`self.OnExecuted` null))))

(event `OnProgramExecuted_Event` :!signature `self.OnExecuted`
  (params (Result :type "/Game/BPSLang/AST/BP_ASTNode Object Reference") (Success :type Boolean))
  ;[1 1 1] Passing args and executing
  (remove `self.OnExecuted` (stale `OnProgCallIDExec_Event` _asbp_astnode_program) (delegate `OnProgramExecuted_Event`))
  (if Success
    (if (`self.Duplicating`)
      (`KismetSystemLibrary.PrintString` null "Program call running duplication" false)
      (else
        (`self.OnExecuted` Result true)))
    (else
      (`KismetSystemLibrary.PrintString` null "Program execution failed or invalid token")
      (`self.OnExecuted` null))))