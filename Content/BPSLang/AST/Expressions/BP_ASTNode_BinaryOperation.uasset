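; AST node for BPSLang, a Blueprint-built scripting language, that evaluates binary operator expressions.
; Evaluate resolves both child nodes, tolerating an unresolved left identifier, then switches on the operator token.
; Arithmetic, append and logical operators build literal tokens from string values, with arithmetic typed by the left operand.
; Assignment stores the right node in program memory, colon sets types, and dot/@ look up nested program fields, @ also evaluating them.
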(fn `Evaluate`
  (params (Origin :type String))
  (returns (Token :type "/Game/BPSLang/Token/BP_SLang_Token Object Reference") (Success :type Boolean))
  (locals (TmpValue :type String) (OpType :type Integer) (ProgramFieldResolve :type Boolean))
  (bind _lefttok (`self.LeftTok`))
  (bind _lefttok_2 (`self.LeftTok`))
  (bind _lefttok_3 (`self.LeftTok`))
  (bind _lefttok_4 (`self.LeftTok`))
  (bind _type (`/Game/BPSLang/Token/BP_SLang_Token.Type` (`self.RightTok`)))
  (bind _value (`/Game/BPSLang/Token/BP_SLang_Token.Value` (`self.RightTok`)))
  (bind _type_2 (`/Game/BPSLang/Token/BP_SLang_Token.Type` (`self.RightTok`)))
  (bind _type_3 (`/Game/BPSLang/Token/BP_SLang_Token.Type` (`self.LeftTok`)))
  (bind _programcontext (`/Game/BPSLang/AST/BP_ASTNode.ProgramContext` (`self.Left`)))
  (bind _type_4 (`/Game/BPSLang/Token/BP_SLang_Token.Type` _lefttok_4))
  (bind (_value_2 _returnvalue) (`BlueprintMapLibrary.Map_Find` (`/Game/BPSLang/AST/BP_ASTNode_Program.Memory` (`self.ProgramContext`)) (`/Game/BPSLang/Token/BP_SLang_Token.Value` _lefttok_3)))
  (bind _returnvalue_2 (`KismetStringLibrary.Conv_StringToDouble` (`/Game/BPSLang/Token/BP_SLang_Token.Value` (`self.RightTok`))))
  (bind _returnvalue_3 (`KismetStringLibrary.Conv_StringToDouble` (`/Game/BPSLang/Token/BP_SLang_Token.Value` (`self.LeftTok`))))
  (bind _returnvalue_4 (> (`KismetStringLibrary.Conv_StringToDouble` (`/Game/BPSLang/Token/BP_SLang_Token.Value` (`self.RightTok`))) 0.0))
  (bind _returnvalue_5 (> (`KismetStringLibrary.Conv_StringToDouble` (`/Game/BPSLang/Token/BP_SLang_Token.Value` (`self.LeftTok`))) 0.0))
  (bind _returnvalue_6 (select `int` (`local.OpType`) :`0` (+ _returnvalue_3 _returnvalue_2) :`1` (- _returnvalue_3 _returnvalue_2) :`2` (* _returnvalue_3 _returnvalue_2) :`3` (/ _returnvalue_3 _returnvalue_2) :`4` (`KismetMathLibrary.MultiplyMultiply_FloatFloat` _returnvalue_3 _returnvalue_2)))
  (`KismetSystemLibrary.PrintString` null (`KismetStringLibrary.Concat_StrStr` "Running Binary operation from " Origin " | Current operator: " (`/Game/BPSLang/Token/BP_SLang_Token.Value` (`self.IdentityToken`))) false)
  ;[1 1 1] Save left token, if it doesn't evaluate and it's ID, make this an assignment
  (bind _left (`self.Left`)
    (:`then`
      (bind (_token _success) (`self.Evaluate` _left "BinaryLeft"))
      (set `self.LeftTok` _token)
      (if _success
        _
        (elif (`|EnumEquality` (`/Game/BPSLang/Token/BP_SLang_Token.Domain` _token) "NewEnumerator1")
          _
          (else
            (`KismetSystemLibrary.PrintString` null "Left did not evaluate and is not an ID" false)
            (return null false))))
      ;[1 1 1] Save Right token
      (bind _right (`self.Right`)
        (:`then`
          (bind (_token_2 _success_2) (`self.Evaluate` _right "BinaryRight"))
          (if _success_2
            (set `self.RightTok` _token_2)
            (switch `string` (`/Game/BPSLang/Token/BP_SLang_Token.Value` (`self.IdentityToken`))
              (:`Default`
                ;[1 1 1] Operator Not Found
                (`KismetSystemLibrary.PrintString` null "Binary can't switch on operator" false)
                (return null false))
              (:`=`
                ;[1 1 1] Assignment
                (if (or (`KismetStringLibrary.EqualEqual_StrStr` _type _type_4) (`KismetStringLibrary.IsEmpty` _type_4))
                  (set `/Game/BPSLang/Token/BP_SLang_Token.Type` _type _lefttok_4)
                  (`BlueprintMapLibrary.Map_Add` (`/Game/BPSLang/AST/BP_ASTNode_Program.Memory` _programcontext) (`/Game/BPSLang/Token/BP_SLang_Token.Value` _lefttok_4) (`self.Right`))
                  (`KismetSystemLibrary.PrintString` null (`KismetStringLibrary.Concat_StrStr` "Assigning variable in program context: " (`/Game/BPSLang/AST/BP_ASTNode_Program.ProgramName` _programcontext)))
                  (return (`self.RightTok`) true)
                  (else
                    (`KismetSystemLibrary.PrintString` null "Assignment type mismatch")
                    (return null false))))
              (:`+`
                (set `local.OpType` 0))
              (:`-`
                (set `local.OpType` 1))
              (:`*`
                (set `local.OpType` 2))
              (:`/`
                (set `local.OpType` 3))
              (:`^`
                (set `local.OpType` 4))
              (:`&`
                ;[1 1 1] Appending
                (bind _returnvalue_7 (`|GenericCreateObject` "/Game/BPSLang/Token/BP_SLang_Token.BP_SLang_Token_C"))
                (`/Game/BPSLang/Token/BP_SLang_Token.MakeLiteral` _returnvalue_7 (`KismetStringLibrary.Concat_StrStr` (`/Game/BPSLang/Token/BP_SLang_Token.Value` _lefttok) (`/Game/BPSLang/Token/BP_SLang_Token.Value` (`self.RightTok`))) (`/Game/BPSLang/Token/BP_SLang_Token.Type` _lefttok))
                (return _returnvalue_7 true))
              (:`&&`
                ;[1 1 1] Logicals
                (bind _returnvalue_8 (`|GenericCreateObject` "/Game/BPSLang/Token/BP_SLang_Token.BP_SLang_Token_C"))
                (`/Game/BPSLang/Token/BP_SLang_Token.MakeLiteral` _returnvalue_8 (select `bool` (and _returnvalue_5 _returnvalue_4) :`false` "0" :`true` "1") "int")
                (return _returnvalue_8 true))
              (:`||`
                (bind _returnvalue_9 (`|GenericCreateObject` "/Game/BPSLang/Token/BP_SLang_Token.BP_SLang_Token_C"))
                (`/Game/BPSLang/Token/BP_SLang_Token.MakeLiteral` _returnvalue_9 (select `bool` (or _returnvalue_5 _returnvalue_4) :`false` "0" :`true` "1") "int")
                (return _returnvalue_9 true))
              (:`:`
                ;[1 1 1] Type assignment
                (if (and (`|EnumEquality` (`/Game/BPSLang/Token/BP_SLang_Token.Domain` (`self.LeftTok`)) "NewEnumerator1") (`|EnumEquality` (`/Game/BPSLang/Token/BP_SLang_Token.Domain` (`self.RightTok`)) "NewEnumerator5"))
                  (bind _output_get (set `/Game/BPSLang/Token/BP_SLang_Token.Type` (`/Game/BPSLang/Token/BP_SLang_Token.Type` (`self.RightTok`)) _lefttok_2))
                  (`KismetSystemLibrary.PrintString` null (`KismetStringLibrary.Concat_StrStr` "Setting token identifier: " _output_get " | Value : " (`/Game/BPSLang/Token/BP_SLang_Token.Value` _lefttok_2)))
                  (return (`self.LeftTok`) true)
                  (else
                    (`KismetSystemLibrary.PrintString` null "Unexpected type assignment" false)
                    (return null false))))
              (:`.`
                ;[1 1 1] Program Fields
                (if (`|EnumEquality` (`/Game/BPSLang/Token/BP_SLang_Token.Domain` _lefttok_3) "NewEnumerator1") :!label _label
                  (if _returnvalue
                    (bind _asbp_astnode_program (cast `/Game/BPSLang/AST/BP_ASTNode_Program` _value_2)
                      (:`then`
                        (bind _memory (`/Game/BPSLang/AST/BP_ASTNode_Program.Memory` _asbp_astnode_program))
                        (bind (_value_3 _returnvalue_10) (`BlueprintMapLibrary.Map_Find` _memory _value))
                        (if _returnvalue_10
                          (set `self.ProgramContext` (`/Game/BPSLang/AST/BP_ASTNode.ProgramContext` _value_3))
                          (if (`local.ProgramFieldResolve`)
                            (bind (_token_3 _success_3) (`self.Evaluate` _value_3 "Binary"))
                            (return _token_3 _success_3)
                            (else
                              (return (`self.RightTok`) true)))
                          (else
                            (`KismetSystemLibrary.PrintString` null (`KismetStringLibrary.Concat_StrStr` "Value not found in program memory: " _value " | Program mem len: " (`KismetStringLibrary.Conv_IntToString` (`BlueprintMapLibrary.Map_Length` _memory))))
                            (return null false))))
                      (:`CastFailed`
                        (`KismetSystemLibrary.PrintString` null "Token not a program")
                        (return null false)))
                    (else
                      (`KismetSystemLibrary.PrintString` null "Left token value not found in memory")
                      (return null false)))
                  (else
                    (`KismetSystemLibrary.PrintString` null "Left token was not identifier")
                    (return null false))))
              (:`@`
                (set `local.ProgramFieldResolve` true)
                (goto _label)))
            ;[1 1 1] Arithmetic
            (if (and (or (`KismetStringLibrary.EqualEqual_StrStr` _type_3 "int") (`KismetStringLibrary.EqualEqual_StrStr` _type_3 "float")) (or (`KismetStringLibrary.EqualEqual_StrStr` _type_2 "int") (`KismetStringLibrary.EqualEqual_StrStr` _type_2 "float")))
              (switch `string` (`/Game/BPSLang/Token/BP_SLang_Token.Type` (`self.LeftTok`))
                (:`Default`
                  (return null false))
                (:`int`
                  (set `local.TmpValue` (`KismetStringLibrary.Conv_IntToString` (`KismetMathLibrary.FTrunc` _returnvalue_6))))
                (:`float`
                  (set `local.TmpValue` (`KismetStringLibrary.Conv_DoubleToString` _returnvalue_6))))
              (bind _returnvalue_11 (`|GenericCreateObject` "/Game/BPSLang/Token/BP_SLang_Token.BP_SLang_Token_C"))
              (`/Game/BPSLang/Token/BP_SLang_Token.MakeLiteral` _returnvalue_11 (`local.TmpValue`) (`/Game/BPSLang/Token/BP_SLang_Token.Type` (`self.LeftTok`)))
              (return _returnvalue_11 true)
              (else
                (return null false)))
            (else
              (`KismetSystemLibrary.PrintString` null "Right did not evaluate" false)
              (return null false))))
        (:`else`
          (`KismetSystemLibrary.PrintString` null "Right Node was not valid" false)
          (return null false))))
    (:`else`
      (`KismetSystemLibrary.PrintString` null "Left Node was not valid" false)
      (return null false))))