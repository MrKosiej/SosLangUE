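; AST node for unary operations in a Blueprint-built scripting language, evaluating negation, logical NOT and return.
; Evaluate switches on the identity token, recursively evaluates the child expression, and builds a new literal token with the result.
; Negation handles only Int and Float operands, while NOT yields an int 1 or 0 from a zero test.
; Return passes the child's token through with its flow-control type set, and unknown operators fail.
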(fn `Evaluate`
  (params (Origin :type String))
  (returns (Token :type "/Game/BPSLang/Token/BP_SLang_Token Object Reference") (Success :type Boolean))
  (locals (TmpValue :type String))
  (switch `string` (`/Game/BPSLang/Token/BP_SLang_Token.Value` (`self.IdentityToken`))
    (:`Default`
      (`KismetSystemLibrary.PrintString` null "Unary not found operator")
      (return null false))
    (:`-`
      ;[1 1 1] Negate
      (bind (_token _success) (`self.Evaluate` (`self.Expression`) "Unary"))
      (if _success
        (switch `/Game/BPSLang/E_TokenOperativeness` (`/Game/BPSLang/Token/BP_SLang_Token.GetOperativeness` _token)
          (:`NewEnumerator0`
            (bind _type (`/Game/BPSLang/Token/BP_SLang_Token.Type` _token))
            (switch `string` _type
              (:`Default`
                (return null false))
              (:`int`
                (bind _value (`/Game/BPSLang/Token/BP_SLang_Token.Value` _token))
                (set `local.TmpValue` (`KismetStringLibrary.Conv_IntToString` (* (`KismetStringLibrary.Conv_StringToInt` _value) -1))))
              (:`float`
                (set `local.TmpValue` (`KismetStringLibrary.Conv_DoubleToString` (* (`KismetStringLibrary.Conv_StringToDouble` _value) -1.0)))))
            (bind _returnvalue (`|GenericCreateObject` "/Game/BPSLang/Token/BP_SLang_Token.BP_SLang_Token_C"))
            (`/Game/BPSLang/Token/BP_SLang_Token.MakeLiteral` _returnvalue (`local.TmpValue`) _type)
            (return _returnvalue true))
          (:`NewEnumerator1`
            _)
          (:`NewEnumerator2`
            _))
        (return null false)
        (else
          (return null false))))
    (:`!`
      ;[1 1 1] NOT
      (bind (_token_2 _success_2) (`self.Evaluate` (`self.Expression`) "Unary"))
      (if _success_2
        (bind _returnvalue_2 (`|GenericCreateObject` "/Game/BPSLang/Token/BP_SLang_Token.BP_SLang_Token_C"))
        (`/Game/BPSLang/Token/BP_SLang_Token.MakeLiteral` _returnvalue_2 (select `bool` (== (`KismetStringLibrary.Conv_StringToDouble` (`/Game/BPSLang/Token/BP_SLang_Token.Value` _token_2)) 0.0) :`false` "0" :`true` "1") "int")
        (return _returnvalue_2 true)
        (else
          (return null false))))
    (:`return`
      ;[1 1 1] Return
      (bind (_token_3 _success_3) (`self.Evaluate` (`self.Expression`) "Unary"))
      (set `/Game/BPSLang/Token/BP_SLang_Token.Flow Control Type` "NewEnumerator1" _token_3)
      (return _token_3 _success_3))))