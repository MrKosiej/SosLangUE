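; AST expression node for the BPSLang Blueprint scripting language that calls a named function outside the script.
; It executes its FunctionName child node and waits for that node's OnExecuted callback.
; On a valid token, it hands the name, arguments and itself to the program's OutsideContext through OutsideExecute.
; An invalid or unsuccessful name prints an error and reports failure.
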(event `self.Execute`
  (params (Origin :type String))
  (bind _functionname (`self.FunctionName`))
  (add `self.OnExecuted` _functionname (delegate `OnFunctionNameExecuted_Event`))
  (`self.Execute` _functionname "Function Out Call Name"))

(event `OnFunctionNameExecuted_Event` :!signature `self.OnExecuted`
  (params (Token :type "/Game/BPSLang/Token/BP_SLang_Token Object Reference") (Success :type Boolean))
  (remove `self.OnExecuted` (`self.FunctionName`) (delegate `OnFunctionNameExecuted_Event`))
  (`/Engine/EditorBlueprintResources/StandardMacros.IsValid` Token
    (:`Is Valid`
      (if Success
        (`/Game/BPSLang/BPI_BPSlangIntegration.OutsideExecute` (`/Game/BPSLang/AST/BP_ASTNode_Program.OutsideContext` (`self.ProgramContext`)) (`/Game/BPSLang/Token/BP_SLang_Token.Value` Token) (`self.Args`) self)
        (else
          (`KismetSystemLibrary.PrintString` null "Out Call Name Node invalid or unsuccessful" :!label _label)
          (`self.OnExecuted` null))))
    (:`Is Not Valid`
      (goto _label))))