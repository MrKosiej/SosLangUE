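; AST node for the BPSLang scripting language that executes While, For and If control structures.
; Execute loads the body into a nested program, then evaluates the first argument through a bind-execute-unbind callback chain.
; While and If run the body on a positive value; For treats the value as an iteration count.
; Loops re-evaluate the argument after each body completion, and normal completion returns an int token of 1.
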(event `ReevaluateArgument`
  (bind _output (`|GetArrayItem` (`self.Args`)))
  ;[1 1 1] Arg Eval
  (`/Engine/EditorBlueprintResources/StandardMacros.IncrementInt` (`self.Iterator`) :!label _label
    (:`  `
      (add `self.OnExecuted` _output (delegate `OnArgExeEvent`))
      (`self.Execute` _output "Control Structure"))))

(event `self.Execute`
  (params (Origin :type String))
  ;[1 1 1] Arg Eval
  (set `self.ProgramContext` (`/Game/BPSLang/AST/BP_ASTNode.ProgramContext` (`self.DeclaredProgram`)))
  (set `/Game/BPSLang/AST/BP_ASTNode_Program.Expressions` (`/Game/BPSLang/AST/BP_ASTNode_ExpressionsWrapper.Expressions` (`self.Body`)) (`self.DeclaredProgram`))
  (set `self.Iterator` 0)
  (goto _label))

(event `OnArgExeEvent` :!signature `self.OnExecuted`
  (params (Token :type "/Game/BPSLang/Token/BP_SLang_Token Object Reference") (Success :type Boolean))
  (bind _declaredprogram (`self.DeclaredProgram`))
  (bind _value (`/Game/BPSLang/Token/BP_SLang_Token.GetStandardDetails` (`self.IdentityToken`)))
  ;[1 1 1] Arg Eval
  (remove `self.OnExecuted` (`|GetArrayItem` (`self.Args`)) (delegate `OnArgExeEvent`))
  (`/Engine/EditorBlueprintResources/StandardMacros.IsValid` Token
    (:`Is Valid`
      (if Success
        (`KismetSystemLibrary.PrintString` null (`KismetStringLibrary.Concat_StrStr` "Running Control Struct: " _value))
        (switch `string` _value
          (:`while`
            (if (> (`KismetStringLibrary.Conv_StringToInt` (`/Game/BPSLang/Token/BP_SLang_Token.GetStandardDetails` Token)) 0) :!label _label_2
              ;[1 1 1] While/ If
              (add `self.OnExecuted` _declaredprogram (delegate `OnWhileLoopProgExecuted_Event`) :!label _label_3)
              (`self.Execute` _declaredprogram "Loopers")
              (else
                (bind _returnvalue (`|GenericCreateObject` "/Game/BPSLang/Token/BP_SLang_Token.BP_SLang_Token_C" :!label _label_4))
                (`/Game/BPSLang/Token/BP_SLang_Token.MakeStandardToken` _returnvalue "1" "int" "NewEnumerator4")
                (`self.OnExecuted` _returnvalue true))))
          (:`for`
            (if (<= (`self.Iterator`) (`KismetStringLibrary.Conv_StringToInt` (`/Game/BPSLang/Token/BP_SLang_Token.GetStandardDetails` Token)))
              (goto _label_3)
              (else
                (goto _label_4))))
          (:`if`
            (goto _label_2)))
        (else
          (`KismetSystemLibrary.PrintString` null "Argument invalid token or did not execute well" false :!label _label_5)
          (`self.OnExecuted` null))))
    (:`Is Not Valid`
      (goto _label_5))))

(event `OnWhileLoopProgExecuted_Event` :!signature `self.OnExecuted`
  (params (Token :type "/Game/BPSLang/Token/BP_SLang_Token Object Reference") (Success :type Boolean))
  ;[1 1 1] While/ If
  (remove `self.OnExecuted` (`self.DeclaredProgram`) (delegate `OnWhileLoopProgExecuted_Event`))
  (switch `string` (`/Game/BPSLang/Token/BP_SLang_Token.GetStandardDetails` (`self.IdentityToken`))
    (:`while`
      _)
    (:`for`
      _)
    (:`if`
      (goto _label_4)))
  (`self.ReevaluateArgument`))