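; AST node for unary operations in the in-game SLang scripting language: negate, not, @ lookup, increment, decrement, Return and Wait.
; Execute evaluates the child Expression through an OnExecuted callback, then dispatches on the operator token to produce a result token.
; Lookup and inc/dec search Memory up the parent program contexts; inc/dec stores the result back as a new Literal node.
; Return and Wait tag the token's flow-control type, and most failures print an error.
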(event `AsNegate`
  (bind _executedexpressiontoken (`self.ExecutedExpressionToken`))
  (bind _value (`/Game/BPSLang/Token/BP_SLang_Token.Value` _executedexpressiontoken))
  (bind _type (`/Game/BPSLang/Token/BP_SLang_Token.Type` _executedexpressiontoken))
  ;[1 1 1] Negate
  (switch `/Game/BPSLang/E_TokenOperativeness` (`/Game/BPSLang/Token/BP_SLang_Token.GetOperativeness` _executedexpressiontoken)
    (:`NewEnumerator0`
      (switch `string` _type
        (:`Default`
          (`KismetSystemLibrary.PrintString` null "Unexpected Type" false)
          (`self.OnExecuted` null))
        (:`int`
          (set `self.TmpValue` (`KismetStringLibrary.Conv_IntToString` (* (`KismetStringLibrary.Conv_StringToInt` _value) -1)))
          (bind _returnvalue (`|GenericCreateObject` "/Game/BPSLang/Token/BP_SLang_Token.BP_SLang_Token_C" :!label _label))
          (`/Game/BPSLang/Token/BP_SLang_Token.MakeStandardToken` _returnvalue (`self.TmpValue`) _type (`/Game/BPSLang/Token/BP_SLang_Token.Domain` (`self.ExecutedExpressionToken`)))
          (`self.OnExecuted` _returnvalue true))
        (:`float`
          (set `self.TmpValue` (`KismetStringLibrary.Conv_DoubleToString` (* (`KismetStringLibrary.Conv_StringToDouble` _value) -1.0)))
          (goto _label))))
    (:`NewEnumerator1`
      (`KismetSystemLibrary.PrintString` null "Unexpected Operativeness" false :!label _label_2)
      (`self.OnExecuted` null))
    (:`NewEnumerator2`
      (goto _label_2))))

(event `AsIncrement`
  (bind _currentprogramcontext (`self.CurrentProgramContext`))
  (bind _value (`/Game/BPSLang/Token/BP_SLang_Token.Value` (`self.ExecutedExpressionToken`)))
  (bind (_value_2 _returnvalue) (`BlueprintMapLibrary.Map_Find` (`/Game/BPSLang/AST/BP_ASTNode_Program.Memory` _currentprogramcontext) _value))
  ;[1 1 1] Inc Dec
  (set `self.Incrementing` true)
  (`self.CurrentProgramContext` :!label _label_3
    (:`then`
      (if _returnvalue :!label _label_4
        (add `self.OnExecuted` _value_2 (delegate `OnIncVarFound`))
        (`self.Execute` _value_2 "Unary")
        (else
          (bind _programcontext (`/Game/BPSLang/AST/BP_ASTNode.ProgramContext` _currentprogramcontext)
            (:`then`
              (set `self.CurrentProgramContext` _programcontext)
              (goto _label_4))
            (:`else`
              (`KismetSystemLibrary.PrintString` null (`KismetStringLibrary.Concat_StrStr` "Did not find ( " _value " ) in program context with name: " (`/Game/BPSLang/AST/BP_ASTNode_Program.ProgramName` _currentprogramcontext)) false :!label _label_5)
              (`self.OnExecuted` null))))))
    (:`else`
      (goto _label_5))))

(event `AsDecrement`
  ;[1 1 1] Inc Dec
  (set `self.Incrementing` false)
  (goto _label_3))

(event `OnIncVarFound` :!signature `self.OnExecuted`
  (params (Token :type "/Game/BPSLang/Token/BP_SLang_Token Object Reference") (Success :type Boolean))
  (bind (_value _type _domain) (`/Game/BPSLang/Token/BP_SLang_Token.GetStandardDetails` Token))
  (bind _returnvalue (`KismetStringLibrary.Conv_StringToInt` (`/Game/BPSLang/Token/BP_SLang_Token.Value` Token)))
  ;[1 1 1] Inc Dec
  (remove `self.OnExecuted` (`BlueprintMapLibrary.Map_Find` (`/Game/BPSLang/AST/BP_ASTNode_Program.Memory` (`self.CurrentProgramContext`)) (`/Game/BPSLang/Token/BP_SLang_Token.Value` (`self.ExecutedExpressionToken`))) (delegate `OnIncVarFound`))
  (`/Engine/EditorBlueprintResources/StandardMacros.IsValid` Token
    (:`Is Valid`
      (if Success
        (if (`self.Incrementing`)
          (bind _result (`/Engine/EditorBlueprintResources/StandardMacros.IncrementInt` _returnvalue)
            (:`  `
              _))
          (else
            (bind _result_2 (`/Engine/EditorBlueprintResources/StandardMacros.DecrementInt` _returnvalue)
              (:`  `
                _))))
        (bind _returnvalue_2 (`|GenericCreateObject` "/Game/BPSLang/Token/BP_SLang_Token.BP_SLang_Token_C"))
        (`/Game/BPSLang/Token/BP_SLang_Token.MakeStandardToken` _returnvalue_2 (`KismetStringLibrary.Conv_IntToString` (select `bool` (`self.Incrementing`) :`false` _result_2 :`true` _result)) _type _domain)
        (bind _returnvalue_3 (`|GenericCreateObject` "/Game/BPSLang/AST/Expressions/BP_ASTNode_Literal.BP_ASTNode_Literal_C" (`self.CurrentProgramContext`) _returnvalue_2))
        (`BlueprintMapLibrary.Map_Add` (`/Game/BPSLang/AST/BP_ASTNode_Program.Memory` (`self.CurrentProgramContext`)) (`/Game/BPSLang/Token/BP_SLang_Token.Value` (`self.ExecutedExpressionToken`)) _returnvalue_3)
        (`self.OnExecuted` _returnvalue_2 true)
        (else
          (`KismetSystemLibrary.PrintString` null "Inc Execution Token not valid or failed" false :!label _label_6)
          (`self.OnExecuted` null))))
    (:`Is Not Valid`
      (goto _label_6))))

(event `AsNot`
  ;[1 1 1] NOT
  (bind _returnvalue (`|GenericCreateObject` "/Game/BPSLang/Token/BP_SLang_Token.BP_SLang_Token_C"))
  (`/Game/BPSLang/Token/BP_SLang_Token.MakeStandardToken` _returnvalue (select `bool` (== (`KismetStringLibrary.Conv_StringToDouble` (`/Game/BPSLang/Token/BP_SLang_Token.Value` (`self.ExecutedExpressionToken`))) 0.0) :`false` "0" :`true` "1") "int" "NewEnumerator4")
  (`self.OnExecuted` _returnvalue true))

(event `AsReturn`
  (bind _executedexpressiontoken (`self.ExecutedExpressionToken`))
  ;[1 1 1] Return
  (set `/Game/BPSLang/Token/BP_SLang_Token.Flow Control Type` "NewEnumerator1" _executedexpressiontoken)
  (`self.OnExecuted` _executedexpressiontoken true))

(event `AsWait`
  (bind _executedexpressiontoken (`self.ExecutedExpressionToken`))
  ;[1 1 1] Wait
  (set `/Game/BPSLang/Token/BP_SLang_Token.Flow Control Type` "NewEnumerator4" _executedexpressiontoken)
  (`self.OnExecuted` _executedexpressiontoken true))

(event `self.Execute`
  (params (Origin :type String))
  (bind _expression (`self.Expression`))
  ;[1 1 1] Init
  (set `self.CurrentProgramContext` (`/Game/BPSLang/AST/BP_ASTNode.ProgramContext` (`self.Expression`)))
  (set `self.ExecutedExpressionToken` null)
  (set `self.TmpValue` "")
  ;[1 1 1] Resolve Expression
  (add `self.OnExecuted` _expression (delegate `OnExpressionExecuted_Event`))
  (`self.Execute` _expression "Unary"))

(event `OnExpressionExecuted_Event` :!signature `self.OnExecuted`
  (params (Token :type "/Game/BPSLang/Token/BP_SLang_Token Object Reference") (Success :type Boolean))
  ;[1 1 1] Resolve Expression
  (remove `self.OnExecuted` (`self.Expression`) (delegate `OnExpressionExecuted_Event`))
  (`/Engine/EditorBlueprintResources/StandardMacros.IsValid` Token
    (:`Is Valid`
      (if Success
        (set `self.ExecutedExpressionToken` Token)
        ;[1 1 1] Switch on Operand
        (switch `string` (`/Game/BPSLang/Token/BP_SLang_Token.Value` (`self.IdentityToken`))
          (:`-`
            (`self.AsNegate`))
          (:`!`
            (`self.AsNot`))
          (:`@`
            (`self.AsAt`))
          (:`return`
            (`self.AsReturn`))
          (:`wait`
            (`self.AsWait`))
          (:`++`
            (`self.AsIncrement`))
          (:`--`
            (`self.AsDecrement`)))
        (else
          (`KismetSystemLibrary.PrintString` null "Expression Failed to Execute" false)
          (`self.OnExecuted` null))))
    (:`Is Not Valid`
      (`KismetSystemLibrary.PrintString` null "Expression Exec Token Not Valid" false)
      (`self.OnExecuted` null))))

(event `AsAt`
  (bind _value (`/Game/BPSLang/Token/BP_SLang_Token.Value` (`self.ExecutedExpressionToken`)))
  ;[1 1 1] At
  (bind _currentprogramcontext (`self.CurrentProgramContext`)
    (:`then`
      (bind (_value_2 _returnvalue) (`BlueprintMapLibrary.Map_Find` (`/Game/BPSLang/AST/BP_ASTNode_Program.Memory` _currentprogramcontext) _value))
      (if _returnvalue :!label _label_7
        (add `self.OnExecuted` _value_2 (delegate `OnAtExecuted_Event`))
        (`self.Execute` _value_2 "Unary")
        (else
          (bind _programcontext (`/Game/BPSLang/AST/BP_ASTNode.ProgramContext` _currentprogramcontext)
            (:`then`
              (set `self.CurrentProgramContext` _programcontext)
              (goto _label_7))
            (:`else`
              (`KismetSystemLibrary.PrintString` null (`KismetStringLibrary.Concat_StrStr` "Did not find ( " _value " ) in program context with name: " (`/Game/BPSLang/AST/BP_ASTNode_Program.ProgramName` _currentprogramcontext)) false :!label _label_8)
              (`self.OnExecuted` null))))))
    (:`else`
      (goto _label_8))))

(event `OnAtExecuted_Event` :!signature `self.OnExecuted`
  (params (Token :type "/Game/BPSLang/Token/BP_SLang_Token Object Reference") (Success :type Boolean))
  (bind (_value _type _domain) (`/Game/BPSLang/Token/BP_SLang_Token.GetStandardDetails` Token))
  ;[1 1 1] At
  (remove `self.OnExecuted` (`BlueprintMapLibrary.Map_Find` (`/Game/BPSLang/AST/BP_ASTNode_Program.Memory` (stale `AsAt` _currentprogramcontext)) (`/Game/BPSLang/Token/BP_SLang_Token.Value` (`self.ExecutedExpressionToken`))) (delegate `OnAtExecuted_Event`))
  (`/Engine/EditorBlueprintResources/StandardMacros.IsValid` Token
    (:`Is Valid`
      (if Success
        (bind _returnvalue (`|GenericCreateObject` "/Game/BPSLang/Token/BP_SLang_Token.BP_SLang_Token_C"))
        (`/Game/BPSLang/Token/BP_SLang_Token.MakeStandardToken` _returnvalue _value _type _domain)
        (`self.OnExecuted` _returnvalue true)
        (else
          (`KismetSystemLibrary.PrintString` null "Failed to eval Token in AT" false)
          (`self.OnExecuted` null))))
    (:`Is Not Valid`
      (`KismetSystemLibrary.PrintString` null "At Execution Token Invalid" false)
      (`self.OnExecuted` null))))