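; AST node for BPSLang, a Blueprint-built scripting language, that evaluates binary arithmetic: add, subtract, multiply, divide and power.
; Execute defers to the parent, then on its ReadyToOperate event maps the operator token to an operation index.
; Numeric operands are computed as doubles, and the result becomes a new literal token of the left operand's type, truncated for int.
; Non-numeric operands print an error and report failure.
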(event `AsArithmetic`
  (bind _type (`/Game/BPSLang/Token/BP_SLang_Token.Type` (`self.RightTok`)))
  (bind _type_2 (`/Game/BPSLang/Token/BP_SLang_Token.Type` (`self.LeftTok`)))
  (bind _returnvalue (`KismetStringLibrary.Conv_StringToDouble` (`/Game/BPSLang/Token/BP_SLang_Token.Value` (`self.RightTok`))))
  (bind _returnvalue_2 (`KismetStringLibrary.Conv_StringToDouble` (`/Game/BPSLang/Token/BP_SLang_Token.Value` (`self.LeftTok`))))
  (bind _returnvalue_3 (select `int` (`self.OpType`) :`0` (+ _returnvalue_2 _returnvalue) :`1` (- _returnvalue_2 _returnvalue) :`2` (* _returnvalue_2 _returnvalue) :`3` (/ _returnvalue_2 _returnvalue) :`4` (`KismetMathLibrary.MultiplyMultiply_FloatFloat` _returnvalue_2 _returnvalue)))
  ;[1 1 1] Arithmetic
  (if (and (or (`KismetStringLibrary.EqualEqual_StrStr` _type_2 "int") (`KismetStringLibrary.EqualEqual_StrStr` _type_2 "float")) (or (`KismetStringLibrary.EqualEqual_StrStr` _type "int") (`KismetStringLibrary.EqualEqual_StrStr` _type "float")))
    (switch `string` (`/Game/BPSLang/Token/BP_SLang_Token.Type` (`self.LeftTok`))
      (:`Default`
        (`KismetSystemLibrary.PrintString` null "Unexpected type for arithmetic" false :!label _label)
        (`self.OnExecuted` null))
      (:`int`
        (set `self.TmpValue` (`KismetStringLibrary.Conv_IntToString` (`KismetMathLibrary.FTrunc` _returnvalue_3)))
        (bind _returnvalue_4 (`|GenericCreateObject` "/Game/BPSLang/Token/BP_SLang_Token.BP_SLang_Token_C" :!label _label_2))
        (`/Game/BPSLang/Token/BP_SLang_Token.MakeLiteral` _returnvalue_4 (`self.TmpValue`) (`/Game/BPSLang/Token/BP_SLang_Token.Type` (`self.LeftTok`)))
        (`self.OnExecuted` _returnvalue_4 true))
      (:`float`
        (set `self.TmpValue` (`KismetStringLibrary.Conv_DoubleToString` _returnvalue_3))
        (goto _label_2)))
    (else
      (goto _label))))

(event `self.Execute`
  (params (Origin :type String))
  (add `self.ReadyToOperate` (delegate `ReadyToOperate_Event`))
  (`parent.Execute` Origin))

(event `ReadyToOperate_Event`
  (clear `self.ReadyToOperate`)
  (switch `string` (`/Game/BPSLang/Token/BP_SLang_Token.Value` (`self.IdentityToken`))
    (:`+`
      (set `self.OpType` 0))
    (:`-`
      (set `self.OpType` 1))
    (:`*`
      (set `self.OpType` 2))
    (:`/`
      (set `self.OpType` 3))
    (:`^`
      (set `self.OpType` 4)))
  (`self.AsArithmetic`))