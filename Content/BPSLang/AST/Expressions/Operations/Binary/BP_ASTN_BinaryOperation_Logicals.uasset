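; Binary-operation AST node for the BPSLang scripting language that evaluates logical AND/OR and comparison operators.
; Execute sets both operand get types, runs the parent evaluation, then maps the operator token to an index once ReadyToOperate fires.
; Logicalize selects the result by that index and returns it as an int "1"/"0" literal node.
; Operands convert to doubles, with positive meaning true, except equality, which compares raw values.
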(event `self.Execute`
  (params (Origin :type String) (ReturnType :type "/Game/BPSLang/E_RefVal Enum" :default "NewEnumerator0"))
  (add `self.ReadyToOperate` (delegate `ReadyToOperate_Event`))
  (set `self.LeftGetType` "NewEnumerator1")
  (set `self.RightGetType` "NewEnumerator1")
  (`parent.Execute` Origin ReturnType))

(event `Logicalize`
  (bind _value (`/Game/BPSLang/AST/BP_ASTNode.Value` (`self.LeftEval`)))
  (bind _value_2 (`/Game/BPSLang/AST/BP_ASTNode.Value` (`self.RightEval`)))
  (bind _returnvalue (`KismetStringLibrary.Conv_StringToDouble` _value))
  (bind _returnvalue_2 (`KismetStringLibrary.Conv_StringToDouble` _value_2))
  (bind _returnvalue_3 (> _returnvalue 0.0))
  (bind _returnvalue_4 (> _returnvalue_2 0.0))
  ;[1 1 1] Logicals
  (bind _returnvalue_5 (`|GenericCreateObject` "/Game/BPSLang/AST/Expressions/BP_ASTNode_Literal.BP_ASTNode_Literal_C" (`self.ProgramContext`)))
  (`self.MakeNode` _returnvalue_5 (select `int` (`self.LogicalOpType`) :`0` (select `bool` (and _returnvalue_3 _returnvalue_4) :`false` "0" :`true` "1") :`1` (select `bool` (or _returnvalue_3 _returnvalue_4) :`false` "0" :`true` "1") :`2` (select `bool` (`KismetStringLibrary.EqualEqual_StrStr` _value _value_2) :`false` "0" :`true` "1") :`3` (select `bool` (> _returnvalue _returnvalue_2) :`false` "0" :`true` "1") :`4` (select `bool` (< _returnvalue _returnvalue_2) :`false` "0" :`true` "1") :`5` (select `bool` (>= _returnvalue _returnvalue_2) :`false` "0" :`true` "1") :`6` (select `bool` (<= _returnvalue _returnvalue_2) :`false` "0" :`true` "1")) "int" "NewEnumerator4")
  (`self.OnExecuted` _returnvalue_5 true))

(event `ReadyToOperate_Event`
  (clear `self.ReadyToOperate`)
  (switch `string` (`self.Value`)
    (:`&&`
      (set `self.LogicalOpType` 0))
    (:`||`
      (set `self.LogicalOpType` 1))
    (:`==`
      (set `self.LogicalOpType` 2))
    (:`>`
      (set `self.LogicalOpType` 3))
    (:`<`
      (set `self.LogicalOpType` 4))
    (:`>=`
      (set `self.LogicalOpType` 5))
    (:`<=`
      (set `self.LogicalOpType` 6)))
  (`self.Logicalize`))