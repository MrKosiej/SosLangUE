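; AST node for the BPSLang interpreter that executes the binary assignment (`=`) and type assignment (`:`) operators.
; Execute picks how each operand is evaluated, then the parent's ReadyToOperate callback dispatches by operator.
; `=` checks or infers type, then walks parent program contexts to update the variable, falling back to the node's own context.
; `:` validates operand domains and sets the left operand's type; failures print and report unsuccessful execution.
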(event `AsAssignment`
  (bind _lefteval (`self.LeftEval`))
  (bind _currentprogramcontext (`self.CurrentProgramContext`))
  (bind _righteval (`self.RightEval`))
  (bind _type (`/Game/BPSLang/AST/BP_ASTNode.Type` _lefteval))
  (bind _type_2 (`/Game/BPSLang/AST/BP_ASTNode.Type` (`self.RightEval`)))
  ;[1 1 1] Assignment
  (if (or (`KismetStringLibrary.EqualEqual_StrStr` _type _type_2) (`KismetStringLibrary.IsEmpty` _type))
    (set `/Game/BPSLang/AST/BP_ASTNode.Type` _type_2 _lefteval)
    (set `self.CurrentProgramContext` (`/Game/BPSLang/AST/BP_ASTNode.ProgramContext` _lefteval))
    (if (not (`.ReturnValue` (`BlueprintMapLibrary.Map_Find` (`/Game/BPSLang/AST/BP_ASTNode_Program.Memory` _currentprogramcontext) (`/Game/BPSLang/AST/BP_ASTNode.Value` _lefteval)))) :!label _label
      (bind _programcontext (`/Game/BPSLang/AST/BP_ASTNode.ProgramContext` _currentprogramcontext)
        (:`then`
          (set `self.CurrentProgramContext` _programcontext)
          (goto _label))
        (:`else`
          (set `self.CurrentProgramContext` (`self.ProgramContext`)))))
    (`BlueprintMapLibrary.Map_Add` (`/Game/BPSLang/AST/BP_ASTNode_Program.Memory` (`self.CurrentProgramContext`)) (`/Game/BPSLang/AST/BP_ASTNode.Value` (`self.LeftEval`)) _righteval)
    (`self.OnExecuted` _righteval true)
    (else
      (`KismetSystemLibrary.PrintString` null "Assignment type mismatch" false)
      (`self.OnExecuted` null))))

(event `self.Execute`
  (params (Origin :type String) (ReturnType :type "/Game/BPSLang/E_RefVal Enum" :default "NewEnumerator0"))
  (add `self.ReadyToOperate` (delegate `ReadyToOperate_Event`))
  (switch `string` (`self.Value`)
    (:`=`
      (set `self.LeftGetType` "NewEnumerator0")
      (set `self.RightGetType` "NewEnumerator1"))
    (:`:`
      (set `self.LeftGetType` "NewEnumerator0")
      (set `self.RightGetType` "NewEnumerator0")))
  (`parent.Execute` Origin ReturnType))

(event `ReadyToOperate_Event`
  (clear `self.ReadyToOperate`)
  (switch `string` (`self.Value`)
    (:`=`
      (`self.AsAssignment`))
    (:`:`
      (`self.AsTypeAssignment`))))

(event `AsTypeAssignment`
  (bind _lefteval (`self.LeftEval`))
  (bind _domain (`/Game/BPSLang/AST/BP_ASTNode.Domain` (`self.RightEval`)))
  ;[1 1 1] Type assignment
  (if (and (`|EnumEquality` (`/Game/BPSLang/AST/BP_ASTNode.Domain` (`self.LeftEval`)) "NewEnumerator1") (or (`|EnumEquality` _domain "NewEnumerator1") (`|EnumEquality` _domain "NewEnumerator5")))
    (set `/Game/BPSLang/AST/BP_ASTNode.Type` (`/Game/BPSLang/AST/BP_ASTNode.Value` (`self.RightEval`)) _lefteval)
    (`self.OnExecuted` _lefteval true)
    (else
      (`KismetSystemLibrary.PrintString` null "Failed type assignment" false)
      (`self.OnExecuted` null))))