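; AST node for binary operations in the BPSLang scripting language, handling the &, . and @ operators.
; Execute evaluates Left then Right through chained OnExecuted delegates, choosing value or reference evaluation per operator.
; It then appends values, resolves a field in a program's Memory, or indexes an array or string, reporting through OnExecuted.
; Duplicate clones both children through a similar callback chain.
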(event `AsAppending`
  (bind _lefteval (`self.LeftEval`))
  (bind (_value _type _domain) (`self.GetIdentity` _lefteval))
  ;[1 1 1] Appending
  (bind _returnvalue (`|GenericCreateObject` (`GameplayStatics.GetObjectClass` _lefteval) (`self.ProgramContext`)))
  (`self.MakeNode` _returnvalue (`KismetStringLibrary.Concat_StrStr` (`/Game/BPSLang/AST/BP_ASTNode.Value` _lefteval) (`/Game/BPSLang/AST/BP_ASTNode.Value` (`self.RightEval`))) _type _domain)
  (`self.OnExecuted` _returnvalue true))

(event `self.Execute`
  (params (Origin :type String) (ReturnType :type "/Game/BPSLang/E_RefVal Enum" :default "NewEnumerator0"))
  ;[1 1 1] Init
  (set `self.Return Type` ReturnType)
  (set `self.CurrentProgramContext` (`self.ProgramContext`))
  (set `self.LeftEval` null)
  (set `self.RightEval` null)
  (set `self.TmpValue` "")
  (switch `string` (`self.Value`)
    (:`Default`
      _)
    (:`&`
      (set `self.LeftGetType` "NewEnumerator1")
      (set `self.RightGetType` "NewEnumerator1"))
    (:`.`
      (set `self.LeftGetType` "NewEnumerator0")
      (set `self.RightGetType` "NewEnumerator0"))
    (:`@`
      (set `self.LeftGetType` "NewEnumerator1")
      (set `self.RightGetType` "NewEnumerator1")))
  ;[1 1 1] Save left token, if it doesn't evaluate and it's ID, make this an assignment
  (bind _left (`self.Left`)
    (:`then`
      (add `self.OnExecuted` _left (delegate `OnLeftExecuted_Event`))
      (`self.Execute` _left "Binary" (`self.LeftGetType`)))
    (:`else`
      (`KismetSystemLibrary.PrintString` null "Left Node was not valid" false)
      (`self.OnExecuted` null))))

(event `OnRightExecuted_Event` :!signature `self.OnExecuted`
  (params (Result :type "/Game/BPSLang/AST/BP_ASTNode Object Reference") (Success :type Boolean))
  ;[1 1 1] Save Right token
  (remove `self.OnExecuted` (stale `OnLeftExecuted_Event` _right) (delegate `OnRightExecuted_Event`))
  (if Success
    (set `self.RightEval` Result)
    (`self.ReadyToOperate`)
    (switch `string` (`self.Value`)
      (:`&`
        (`self.AsAppending`))
      (:`.`
        (`self.AsProgramFieldAccess`))
      (:`@`
        (`self.As At`)))
    (else
      (`KismetSystemLibrary.PrintString` null "Right failed to execute" false)
      (`self.OnExecuted` null))))

(event `OnLeftExecuted_Event` :!signature `self.OnExecuted`
  (params (Result :type "/Game/BPSLang/AST/BP_ASTNode Object Reference") (Success :type Boolean))
  ;[1 1 1] Save left token, if it doesn't evaluate and it's ID, make this an assignment
  (remove `self.OnExecuted` (stale `self.Execute` _left) (delegate `OnLeftExecuted_Event`))
  (if Success
    (set `self.LeftEval` Result)
    ;[1 1 1] Save Right token
    (bind _right (`self.Right`)
      (:`then`
        (add `self.OnExecuted` _right (delegate `OnRightExecuted_Event`))
        (`self.Execute` _right "Binary" (`self.RightGetType`)))
      (:`else`
        (`KismetSystemLibrary.PrintString` null "Right Node was not valid" false)
        (`self.OnExecuted` null)))
    (else
      (`KismetSystemLibrary.PrintString` null "Left Node failed to execute" false)
      (`self.OnExecuted` null))))

(event `AsProgramFieldAccess`
  (bind _lefteval (`self.LeftEval`))
  (bind _righteval (`self.RightEval`))
  (bind _value (`/Game/BPSLang/AST/BP_ASTNode.Value` _righteval))
  (bind (_value_2 _returnvalue) (`BlueprintMapLibrary.Map_Find` (`/Game/BPSLang/AST/BP_ASTNode_Program.Memory` (`/Game/BPSLang/AST/BP_ASTNode.ProgramContext` _lefteval)) (`/Game/BPSLang/AST/BP_ASTNode.Value` _lefteval)))
  ;[1 1 1] Program Fields
  (if (`|EnumEquality` (`/Game/BPSLang/AST/BP_ASTNode.Domain` _lefteval) "NewEnumerator1")
    (if _returnvalue
      (bind _asbp_astnode_program (cast `/Game/BPSLang/AST/BP_ASTNode_Program` _value_2)
        (:`then`
          (set `self.ProgramContext` _asbp_astnode_program)
          (bind _memory (`/Game/BPSLang/AST/BP_ASTNode_Program.Memory` _asbp_astnode_program))
          (bind (_value_3 _returnvalue_2) (`BlueprintMapLibrary.Map_Find` _memory _value))
          (if _returnvalue_2
            (bind _returnvalue_3 (select `/Game/BPSLang/E_RefVal` (`self.Return Type`) :`NewEnumerator0` _righteval :`NewEnumerator1` _value_3))
            (set `/Game/BPSLang/AST/BP_ASTNode.ProgramContext` _asbp_astnode_program _returnvalue_3)
            (bind (_value_4 _type _domain) (`self.GetIdentity` _returnvalue_3))
            (bind _programname (`/Game/BPSLang/AST/BP_ASTNode_Program.ProgramName` _asbp_astnode_program))
            (`KismetSystemLibrary.PrintString` null (`KismetStringLibrary.Concat_StrStr` "field access returning: " _value_4 " | " _type " | " (`|GetEnumeratorNameAsString` _domain) " | From: " _programname))
            (`self.OnExecuted` _returnvalue_3 true)
            (else
              (`KismetSystemLibrary.PrintString` null (`KismetStringLibrary.Concat_StrStr` "Value not found in program memory: " _value " | Program mem len: " (`KismetStringLibrary.Conv_IntToString` (`BlueprintMapLibrary.Map_Length` _memory)) " | Program Name: " _programname) false)
              (`self.OnExecuted` null))))
        (:`CastFailed`
          (`KismetSystemLibrary.PrintString` null (`KismetStringLibrary.Concat_StrStr` "Token not a program, it's : " (`KismetSystemLibrary.GetDisplayName` _value_2)) false)
          (`self.OnExecuted` null)))
      (else
        (`KismetSystemLibrary.PrintString` null "Left token value not found in memory" false)
        (`self.OnExecuted` null)))
    (else
      (`KismetSystemLibrary.PrintString` null "Left token was not identifier" false)
      (`self.OnExecuted` null))))

(event `self.Duplicate`
  (bind _left (`self.Left`))
  ;[1 1 1] Duplicate
  (add `self.OnDuplicated` _left (delegate `OnLeftDuplicated_Event`))
  (`self.Duplicate` _left))

(event `OnLeftDuplicated_Event` :!signature `self.OnDuplicated`
  (params (Duplicate :type "/Game/BPSLang/AST/BP_ASTNode Object Reference"))
  (bind _right (`self.Right`))
  ;[1 1 1] Duplicate
  (remove `self.OnDuplicated` (`self.Left`) (delegate `OnLeftDuplicated_Event`))
  (add `self.OnDuplicated` _right (delegate `OnRightDuplicated_Event`))
  (`self.Duplicate` _right))

(event `OnRightDuplicated_Event` :!signature `self.OnDuplicated`
  (params (Duplicate :type "/Game/BPSLang/AST/BP_ASTNode Object Reference"))
  ;[1 1 1] Duplicate
  (remove `self.OnDuplicated` (`self.Right`) (delegate `OnRightDuplicated_Event`))
  (bind _returnvalue (`|GenericCreateObject` (`GameplayStatics.GetObjectClass` self) (stale `OnLeftDuplicated_Event` Duplicate) Duplicate (`self.ProgramContext`)))
  (`self.OnDuplicated` _returnvalue))

(event `As At`
  (bind _lefteval (`self.LeftEval`))
  (bind (_value _type _domain) (`self.GetIdentity` (`self.LeftEval`)))
  (bind _returnvalue (`KismetStringLibrary.Conv_StringToInt` (`/Game/BPSLang/AST/BP_ASTNode.Value` (`self.RightEval`))))
  (bind _returnvalue_2 (`KismetStringLibrary.GetCharacterArrayFromString` (`/Game/BPSLang/AST/BP_ASTNode.Value` _lefteval)))
  ;[1 1 1] As At
  (bind _asbp_astnode_array (cast `/Game/BPSLang/AST/BP_ASTNode_Array` _lefteval)
    (:`then`
      (bind _nodes (`/Game/BPSLang/AST/BP_ASTNode_Array.Nodes` _asbp_astnode_array))
      (if (`KismetArrayLibrary.Array_IsValidIndex` _nodes _returnvalue)
        (`self.OnExecuted` (`|GetArrayItem` _nodes _returnvalue) true)
        (else
          (`KismetSystemLibrary.PrintString` null "Invalid Array Index" :!label _label)
          (`self.OnExecuted` null))))
    (:`CastFailed`
      (if (`KismetArrayLibrary.Array_IsValidIndex` _returnvalue_2 _returnvalue)
        (bind _returnvalue_3 (`|GenericCreateObject` "/Game/BPSLang/AST/Expressions/BP_ASTNode_Literal.BP_ASTNode_Literal_C" (`self.CurrentProgramContext`)))
        (`self.MakeNode` _returnvalue_3 (`|GetArrayItem` _returnvalue_2 _returnvalue) _type _domain)
        (`self.OnExecuted` _returnvalue_3 true)
        (else
          (goto _label))))))