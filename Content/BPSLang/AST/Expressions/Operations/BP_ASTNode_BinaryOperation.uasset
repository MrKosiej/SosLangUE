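; AST node for a Blueprint-built scripting language that evaluates a binary operation.
; Execute runs the Left then Right child through OnExecuted callbacks, then switches on the operator token.
; Operators cover assignment into program memory, int/float arithmetic, append, logicals, type annotation and dot lookup into another program's memory.
; It reports a resulting token or failure through CallOnExecuted, printing debug messages.
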(event `OnRightExecuted_Event` :!signature `self.OnExecuted`
  (params (Token :type "/Game/BPSLang/Token/BP_SLang_Token Object Reference") (Success :type Boolean))
  (bind _lefttok (`self.LeftTok`))
  (bind _lefttok_2 (`self.LeftTok`))
  (bind _lefttok_3 (`self.LeftTok`))
  (bind _lefttok_4 (`self.LeftTok`))
  (bind (_value _type) (`/Game/BPSLang/Token/BP_SLang_Token.AsLiteral` (`self.RightTok`)))
  (bind _type_2 (`/Game/BPSLang/Token/BP_SLang_Token.Type` (`self.RightTok`)))
  (bind _value_2 (`/Game/BPSLang/Token/BP_SLang_Token.Value` (`self.RightTok`)))
  (bind _type_3 (`/Game/BPSLang/Token/BP_SLang_Token.Type` (`self.RightTok`)))
  (bind _type_4 (`/Game/BPSLang/Token/BP_SLang_Token.Type` (`self.LeftTok`)))
  (bind _type_5 (`/Game/BPSLang/Token/BP_SLang_Token.Type` _lefttok_4))
  (bind _value_3 (`/Game/BPSLang/Token/BP_SLang_Token.Value` (`self.RightTok`)))
  (bind _returnvalue (`KismetStringLibrary.Conv_StringToDouble` (`/Game/BPSLang/Token/BP_SLang_Token.Value` (`self.RightTok`))))
  (bind _returnvalue_2 (`KismetStringLibrary.Conv_StringToDouble` (`/Game/BPSLang/Token/BP_SLang_Token.Value` (`self.LeftTok`))))
  (bind (_value_4 _returnvalue_3) (`BlueprintMapLibrary.Map_Find` (`/Game/BPSLang/AST/BP_ASTNode_Program.Memory` (`/Game/BPSLang/AST/BP_ASTNode.ProgramContext` (`self.Left`))) (`/Game/BPSLang/Token/BP_SLang_Token.Value` _lefttok_3)))
  (bind _returnvalue_4 (> (`KismetStringLibrary.Conv_StringToDouble` (`/Game/BPSLang/Token/BP_SLang_Token.Value` (`self.RightTok`))) 0.0))
  (bind _returnvalue_5 (> (`KismetStringLibrary.Conv_StringToDouble` (`/Game/BPSLang/Token/BP_SLang_Token.Value` (`self.LeftTok`))) 0.0))
  (bind _returnvalue_6 (select `int` (`self.OpType`) :`0` (+ _returnvalue_2 _returnvalue) :`1` (- _returnvalue_2 _returnvalue) :`2` (* _returnvalue_2 _returnvalue) :`3` (/ _returnvalue_2 _returnvalue) :`4` (`KismetMathLibrary.MultiplyMultiply_FloatFloat` _returnvalue_2 _returnvalue)))
  ;[1 1 1] Save Right token
  (`/Engine/EditorBlueprintResources/StandardMacros.IsValid` Token
    (:`Is Valid`
      (if Success
        (set `self.RightTok` Token)
        (switch `string` (`/Game/BPSLang/Token/BP_SLang_Token.Value` (`self.IdentityToken`))
          (:`Default`
            ;[1 1 1] Operator Not Found
            (`KismetSystemLibrary.PrintString` null "Binary can't switch on operator" false)
            (`self.OnExecuted` null))
          (:`=`
            ;[1 1 1] Assignment
            (if (or (`KismetStringLibrary.EqualEqual_StrStr` _type_2 _type_5) (`KismetStringLibrary.IsEmpty` _type_5))
              (set `/Game/BPSLang/Token/BP_SLang_Token.Type` _type_2 _lefttok_4)
              (`BlueprintMapLibrary.Map_Add` (`/Game/BPSLang/AST/BP_ASTNode_Program.Memory` (`/Game/BPSLang/AST/BP_ASTNode.ProgramContext` (`self.Left`))) (`/Game/BPSLang/Token/BP_SLang_Token.Value` _lefttok_4) (`self.Right`))
              (`self.OnExecuted` (`self.RightTok`) true)
              (else
                (`KismetSystemLibrary.PrintString` null "Assignment type mismatch" false)
                (`self.OnExecuted` null))))
          (:`+`
            (set `self.OpType` 0)
            ;[1 1 1] Arithmetic
            (if (and (or (`KismetStringLibrary.EqualEqual_StrStr` _type_4 "int") (`KismetStringLibrary.EqualEqual_StrStr` _type_4 "float")) (or (`KismetStringLibrary.EqualEqual_StrStr` _type_3 "int") (`KismetStringLibrary.EqualEqual_StrStr` _type_3 "float"))) :!label _label
              (switch `string` (`/Game/BPSLang/Token/BP_SLang_Token.Type` (`self.LeftTok`))
                (:`Default`
                  (`KismetSystemLibrary.PrintString` null "Unexpected type for arithmetic" false :!label _label_2)
                  (`self.OnExecuted` null))
                (:`int`
                  (set `self.TmpValue` (`KismetStringLibrary.Conv_IntToString` (`KismetMathLibrary.FTrunc` _returnvalue_6)))
                  (bind _returnvalue_7 (`|GenericCreateObject` "/Game/BPSLang/Token/BP_SLang_Token.BP_SLang_Token_C" :!label _label_3))
                  (`/Game/BPSLang/Token/BP_SLang_Token.MakeLiteral` _returnvalue_7 (`self.TmpValue`) (`/Game/BPSLang/Token/BP_SLang_Token.Type` (`self.LeftTok`)))
                  (`self.OnExecuted` _returnvalue_7 true))
                (:`float`
                  (set `self.TmpValue` (`KismetStringLibrary.Conv_DoubleToString` _returnvalue_6))
                  (goto _label_3)))
              (else
                (goto _label_2))))
          (:`-`
            (set `self.OpType` 1)
            (goto _label))
          (:`*`
            (set `self.OpType` 2)
            (goto _label))
          (:`/`
            (set `self.OpType` 3)
            (goto _label))
          (:`^`
            (set `self.OpType` 4)
            (goto _label))
          (:`&`
            ;[1 1 1] Appending
            (bind _returnvalue_8 (`|GenericCreateObject` "/Game/BPSLang/Token/BP_SLang_Token.BP_SLang_Token_C"))
            (`/Game/BPSLang/Token/BP_SLang_Token.MakeLiteral` _returnvalue_8 (`KismetStringLibrary.Concat_StrStr` (`/Game/BPSLang/Token/BP_SLang_Token.Value` _lefttok) (`/Game/BPSLang/Token/BP_SLang_Token.Value` (`self.RightTok`))) (`/Game/BPSLang/Token/BP_SLang_Token.Type` _lefttok))
            (`self.OnExecuted` _returnvalue_8 true))
          (:`&&`
            ;[1 1 1] Logicals
            (bind _returnvalue_9 (`|GenericCreateObject` "/Game/BPSLang/Token/BP_SLang_Token.BP_SLang_Token_C"))
            (`/Game/BPSLang/Token/BP_SLang_Token.MakeLiteral` _returnvalue_9 (select `bool` (and _returnvalue_5 _returnvalue_4) :`false` "0" :`true` "1") "int")
            (`self.OnExecuted` _returnvalue_9 true))
          (:`||`
            (bind _returnvalue_10 (`|GenericCreateObject` "/Game/BPSLang/Token/BP_SLang_Token.BP_SLang_Token_C"))
            (`/Game/BPSLang/Token/BP_SLang_Token.MakeLiteral` _returnvalue_10 (select `bool` (or _returnvalue_5 _returnvalue_4) :`false` "0" :`true` "1") "int")
            (`self.OnExecuted` _returnvalue_10 true))
          (:`:`
            ;[1 1 1] Type assignment
            (if (and (`|EnumEquality` (`/Game/BPSLang/Token/BP_SLang_Token.Domain` (`self.LeftTok`)) "NewEnumerator1") (`|EnumEquality` (`/Game/BPSLang/Token/BP_SLang_Token.Domain` (`self.RightTok`)) "NewEnumerator5"))
              (set `/Game/BPSLang/Token/BP_SLang_Token.Type` _value_3 _lefttok_2)
              (`KismetSystemLibrary.PrintString` null (`KismetStringLibrary.Concat_StrStr` "Setting ID Type in " (`/Game/BPSLang/AST/BP_ASTNode_Program.ProgramName` (`/Game/BPSLang/AST/BP_ASTNode.ProgramContext` (`self.Left`))) " | Value: " (`/Game/BPSLang/Token/BP_SLang_Token.Value` _lefttok_2) " | Type: " _value_3))
              (`self.OnExecuted` _lefttok_2 true)
              (else
                (`KismetSystemLibrary.PrintString` null "Failed type assignment" false)
                (`self.OnExecuted` null))))
          (:`.`
            ;[1 1 1] Program Fields
            (if (`|EnumEquality` (`/Game/BPSLang/Token/BP_SLang_Token.Domain` _lefttok_3) "NewEnumerator1")
              (if _returnvalue_3
                (bind _asbp_astnode_program (cast `/Game/BPSLang/AST/BP_ASTNode_Program` _value_4)
                  (:`then`
                    (set `self.ProgramContext` _asbp_astnode_program)
                    (bind _memory (`/Game/BPSLang/AST/BP_ASTNode_Program.Memory` _asbp_astnode_program))
                    (if (`.ReturnValue` (`BlueprintMapLibrary.Map_Find` _memory _value_2))
                      (bind _returnvalue_11 (`|GenericCreateObject` "/Game/BPSLang/Token/BP_SLang_Token.BP_SLang_Token_C"))
                      (`/Game/BPSLang/Token/BP_SLang_Token.MakeIdentifier` _returnvalue_11 _value _type)
                      (`self.OnExecuted` _returnvalue_11 true)
                      (else
                        (`KismetSystemLibrary.PrintString` null (`KismetStringLibrary.Concat_StrStr` "Value not found in program memory: " _value_2 " | Program mem len: " (`KismetStringLibrary.Conv_IntToString` (`BlueprintMapLibrary.Map_Length` _memory)) " | Program Name: " (`/Game/BPSLang/AST/BP_ASTNode_Program.ProgramName` _asbp_astnode_program)) false)
                        (`self.OnExecuted` null))))
                  (:`CastFailed`
                    (`KismetSystemLibrary.PrintString` null "Token not a program" false)
                    (`self.OnExecuted` null)))
                (else
                  (`KismetSystemLibrary.PrintString` null "Left token value not found in memory" false)
                  (`self.OnExecuted` null)))
              (else
                (`KismetSystemLibrary.PrintString` null "Left token was not identifier" false)
                (`self.OnExecuted` null)))))
        (else
          (`KismetSystemLibrary.PrintString` null "Right failed to execute" false)
          (`self.OnExecuted` null))))
    (:`Is Not Valid`
      (`KismetSystemLibrary.PrintString` null "Right exec token was not valid" false)
      (`self.OnExecuted` null))))

(event `self.Execute`
  (params (Origin :type String))
  ;[1 1 1] Init
  (set `self.LeftTok` null)
  (set `self.RightTok` null)
  (set `self.OpType` 0)
  (set `self.TmpValue` "")
  (`KismetSystemLibrary.PrintString` null (`KismetStringLibrary.Concat_StrStr` "Running Binary operation from " Origin " | Current operator: " (`/Game/BPSLang/Token/BP_SLang_Token.Value` (`self.IdentityToken`))) false)
  ;[1 1 1] Save left token, if it doesn't evaluate and it's ID, make this an assignment
  (bind _left (`self.Left`)
    (:`then`
      (add `self.OnExecuted` _left (delegate `OnLeftExecuted_Event`))
      (`self.Execute` _left "Binary"))
    (:`else`
      (`KismetSystemLibrary.PrintString` null "Left Node was not valid" false)
      (`self.OnExecuted` null))))

(event `OnLeftExecuted_Event` :!signature `self.OnExecuted`
  (params (Token :type "/Game/BPSLang/Token/BP_SLang_Token Object Reference") (Success :type Boolean))
  ;[1 1 1] Save left token, if it doesn't evaluate and it's ID, make this an assignment
  (remove `self.OnExecuted` (stale `self.Execute` _left) (delegate `OnLeftExecuted_Event`))
  (`/Engine/EditorBlueprintResources/StandardMacros.IsValid` Token
    (:`Is Valid`
      (if Success
        (set `self.LeftTok` Token)
        ;[1 1 1] Save Right token
        (bind _right (`self.Right`)
          (:`then`
            (add `self.OnExecuted` _right (delegate `OnRightExecuted_Event`))
            (`self.Execute` _right "Binary"))
          (:`else`
            (`KismetSystemLibrary.PrintString` null "Right Node was not valid" false)
            (`self.OnExecuted` null)))
        (else
          (`KismetSystemLibrary.PrintString` null "Left Node failed to execute" false)
          (`self.OnExecuted` null))))
    (:`Is Not Valid`
      (`KismetSystemLibrary.PrintString` null "Left Node executed to invalid token" false)
      (`self.OnExecuted` null))))