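; AST node for unary operations in the BPSLang scripting language, handling negate, not, @ lookup, increment, decrement, Return and Wait.
; Execute evaluates the child Expression through OnExecuted callbacks, then dispatches on the operator.
; Lookup and increment/decrement search parent program contexts for the named variable, with increment/decrement storing a new literal where found.
; Return and Wait tag the result's FlowControl, and Duplicate rebuilds the node around a duplicated child.
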(event `AsNegate`
  (bind _executedexpression (`self.ExecutedExpression`))
  (bind _value (`/Game/BPSLang/AST/BP_ASTNode.Value` _executedexpression))
  ;[1 1 1] Negate
  (switch `/Game/BPSLang/E_TokenDomain` (`/Game/BPSLang/AST/BP_ASTNode.Domain` _executedexpression)
    (:`NewEnumerator0`
      (`KismetSystemLibrary.PrintString` null "Unexpected Domain" false :!label _label)
      (`self.OnExecuted` null))
    (:`NewEnumerator4`
      (switch `string` (`/Game/BPSLang/AST/BP_ASTNode.Type` _executedexpression)
        (:`Default`
          (`KismetSystemLibrary.PrintString` null "Unexpected Type" false)
          (`self.OnExecuted` null))
        (:`int`
          (set `self.TmpValue` (`KismetStringLibrary.Conv_IntToString` (* (`KismetStringLibrary.Conv_StringToInt` _value) -1)))
          (bind _returnvalue (`|GenericCreateObject` "/Game/BPSLang/AST/Expressions/BP_ASTNode_Literal.BP_ASTNode_Literal_C" (`self.CurrentProgramContext`) :!label _label_2))
          (`self.MakeNode` _returnvalue (`self.TmpValue`) "int" (`/Game/BPSLang/AST/BP_ASTNode.Domain` (`self.ExecutedExpression`)))
          (`self.OnExecuted` _returnvalue true))
        (:`float`
          (set `self.TmpValue` (`KismetStringLibrary.Conv_DoubleToString` (* (`KismetStringLibrary.Conv_StringToDouble` _value) -1.0)))
          (goto _label_2))))
    (:`NewEnumerator1`
      (goto _label))
    (:`NewEnumerator3`
      (goto _label))
    (:`NewEnumerator5`
      (goto _label))))

(event `AsIncrement`
  (bind _currentprogramcontext (`self.CurrentProgramContext`))
  (bind _value (`/Game/BPSLang/AST/BP_ASTNode.Value` (`self.ExecutedExpression`)))
  (bind (_value_2 _returnvalue) (`BlueprintMapLibrary.Map_Find` (`/Game/BPSLang/AST/BP_ASTNode_Program.Memory` _currentprogramcontext) _value))
  ;[1 1 1] Inc Dec
  (set `self.Incrementing` true)
  (`self.CurrentProgramContext` :!label _label_3
    (:`then`
      (if _returnvalue :!label _label_4
        (add `self.OnExecuted` _value_2 (delegate `OnIncVarFound`))
        (`self.Execute` _value_2 "Unary" "NewEnumerator0")
        (else
          (bind _programcontext (`/Game/BPSLang/AST/BP_ASTNode.ProgramContext` _currentprogramcontext)
            (:`then`
              (set `self.CurrentProgramContext` _programcontext)
              (goto _label_4))
            (:`else`
              (`KismetSystemLibrary.PrintString` null (`KismetStringLibrary.Concat_StrStr` "Did not find ( " _value " ) in program context with name: " (`/Game/BPSLang/AST/BP_ASTNode_Program.ProgramName` _currentprogramcontext)) false :!label _label_5)
              (`self.OnExecuted` null))))))
    (:`else`
      (goto _label_5))))

(event `AsDecrement`
  ;[1 1 1] Inc Dec
  (set `self.Incrementing` false)
  (goto _label_3))

(event `AsNot`
  ;[1 1 1] NOT
  (bind _returnvalue (`|GenericCreateObject` "/Game/BPSLang/AST/Expressions/BP_ASTNode_Literal.BP_ASTNode_Literal_C" (`self.CurrentProgramContext`)))
  (`self.MakeNode` _returnvalue (select `bool` (== (`KismetStringLibrary.Conv_StringToDouble` (`/Game/BPSLang/AST/BP_ASTNode.Value` (`self.ExecutedExpression`))) 0.0) :`false` "0" :`true` "1") "int" "NewEnumerator4")
  (`self.OnExecuted` _returnvalue true))

(event `AsReturn`
  (bind _executedexpression (`self.ExecutedExpression`))
  ;[1 1 1] Return
  (set `/Game/BPSLang/AST/BP_ASTNode.FlowControl` "NewEnumerator1" _executedexpression)
  (`self.OnExecuted` _executedexpression true))

(event `OnIncVarFound` :!signature `self.OnExecuted`
  (params (Result :type "/Game/BPSLang/AST/BP_ASTNode Object Reference") (Success :type Boolean))
  (bind (_value _type _domain) (`self.GetIdentity` (`self.ExecutedExpression`)))
  (bind _returnvalue (`KismetStringLibrary.Conv_StringToInt` (`/Game/BPSLang/AST/BP_ASTNode.Value` Result)))
  ;[1 1 1] Inc Dec
  (remove `self.OnExecuted` (`BlueprintMapLibrary.Map_Find` (`/Game/BPSLang/AST/BP_ASTNode_Program.Memory` (`self.CurrentProgramContext`)) (`/Game/BPSLang/AST/BP_ASTNode.Value` (`self.ExecutedExpression`))) (delegate `OnIncVarFound`))
  (if Success
    (if (`self.Incrementing`)
      (bind _result (`/Engine/EditorBlueprintResources/StandardMacros.IncrementInt` _returnvalue)
        (:`  `
          _))
      (else
        (bind _result_2 (`/Engine/EditorBlueprintResources/StandardMacros.DecrementInt` _returnvalue)
          (:`  `
            _))))
    (bind _returnvalue_2 (`|GenericCreateObject` "/Game/BPSLang/AST/Expressions/BP_ASTNode_Literal.BP_ASTNode_Literal_C" (`self.CurrentProgramContext`)))
    (`self.MakeNode` _returnvalue_2 (`KismetStringLibrary.Conv_IntToString` (select `bool` (`self.Incrementing`) :`false` _result_2 :`true` _result)) _type _domain)
    (`BlueprintMapLibrary.Map_Add` (`/Game/BPSLang/AST/BP_ASTNode_Program.Memory` (`self.CurrentProgramContext`)) (`/Game/BPSLang/AST/BP_ASTNode.Value` (`self.ExecutedExpression`)) _returnvalue_2)
    (`self.OnExecuted` _returnvalue_2 true)
    (else
      (`KismetSystemLibrary.PrintString` null "Inc Execution Token not valid or failed" false)
      (`self.OnExecuted` null))))

(event `AsWait`
  (bind _executedexpression (`self.ExecutedExpression`))
  ;[1 1 1] Wait
  (set `/Game/BPSLang/AST/BP_ASTNode.FlowControl` "NewEnumerator4" _executedexpression)
  (`self.OnExecuted` _executedexpression true))

(event `self.Execute`
  (params (Origin :type String) (ReturnType :type "/Game/BPSLang/E_RefVal Enum" :default "NewEnumerator0"))
  (bind _expression (`self.Expression`))
  ;[1 1 1] Init
  (switch `string` (`self.Value`)
    (:`-`
      (set `self.ResolveExpressionAs` "NewEnumerator1"))
    (:`!`
      (set `self.ResolveExpressionAs` "NewEnumerator1"))
    (:`@`
      (set `self.ResolveExpressionAs` "NewEnumerator0"))
    (:`return`
      (set `self.ResolveExpressionAs` "NewEnumerator1"))
    (:`wait`
      (set `self.ResolveExpressionAs` "NewEnumerator1"))
    (:`++`
      (set `self.ResolveExpressionAs` "NewEnumerator0"))
    (:`--`
      (set `self.ResolveExpressionAs` "NewEnumerator0")))
  (set `self.ExecutedExpression` null)
  (set `self.TmpValue` "")
  ;[1 1 1] Resolve Expression
  (add `self.OnExecuted` _expression (delegate `OnExpressionExecuted_Event`))
  (`self.Execute` _expression "Unary" (`self.ResolveExpressionAs`)))

(event `OnExpressionExecuted_Event` :!signature `self.OnExecuted`
  (params (Result :type "/Game/BPSLang/AST/BP_ASTNode Object Reference") (Success :type Boolean))
  ;[1 1 1] Resolve Expression
  (remove `self.OnExecuted` (`self.Expression`) (delegate `OnExpressionExecuted_Event`))
  (if Success
    (set `self.ExecutedExpression` Result)
    (set `self.CurrentProgramContext` (`/Game/BPSLang/AST/BP_ASTNode.ProgramContext` (`self.Expression`)))
    ;[1 1 1] Switch on Operand
    (switch `string` (`self.Value`)
      (:`-`
        (`self.AsNegate`))
      (:`!`
        (`self.AsNot`))
      (:`@`
        (`self.AsAt`))
      (:`return`
        (`self.AsReturn`))
      (:`wait`
        (`self.AsWait`))
      (:`++`
        (`self.AsIncrement`))
      (:`--`
        (`self.AsDecrement`)))
    (else
      (`KismetSystemLibrary.PrintString` null "Expression Failed to Execute" false)
      (`self.OnExecuted` null))))

(event `AsAt`
  (bind _value (`/Game/BPSLang/AST/BP_ASTNode.Value` (`self.ExecutedExpression`)))
  ;[1 1 1] At
  (bind _currentprogramcontext (`self.CurrentProgramContext`)
    (:`then`
      (bind (_value_2 _returnvalue) (`BlueprintMapLibrary.Map_Find` (`/Game/BPSLang/AST/BP_ASTNode_Program.Memory` _currentprogramcontext) _value))
      (if _returnvalue :!label _label_6
        (add `self.OnExecuted` _value_2 (delegate `OnAtExecuted_Event`))
        (`self.Execute` _value_2 "Unary" "NewEnumerator0")
        (else
          (bind _programcontext (`/Game/BPSLang/AST/BP_ASTNode.ProgramContext` _currentprogramcontext)
            (:`then`
              (set `self.CurrentProgramContext` _programcontext)
              (goto _label_6))
            (:`else`
              (`KismetSystemLibrary.PrintString` null (`KismetStringLibrary.Concat_StrStr` "Did not find ( " _value " ) in program context with name: " (`/Game/BPSLang/AST/BP_ASTNode_Program.ProgramName` _currentprogramcontext)) false :!label _label_7)
              (`self.OnExecuted` null))))))
    (:`else`
      (goto _label_7))))

(event `OnAtExecuted_Event` :!signature `self.OnExecuted`
  (params (Result :type "/Game/BPSLang/AST/BP_ASTNode Object Reference") (Success :type Boolean))
  ;[1 1 1] At
  (remove `self.OnExecuted` (`BlueprintMapLibrary.Map_Find` (`/Game/BPSLang/AST/BP_ASTNode_Program.Memory` (stale `AsAt` _currentprogramcontext)) (`/Game/BPSLang/AST/BP_ASTNode.Value` (`self.ExecutedExpression`))) (delegate `OnAtExecuted_Event`))
  (if Success
    (`self.OnExecuted` Result true)
    (else
      (`KismetSystemLibrary.PrintString` null "Failed to eval Token in AT" false)
      (`self.OnExecuted` null))))

(event `self.Duplicate`
  (bind _expression (`self.Expression`))
  ;[1 1 1] Duplicate
  (add `self.OnDuplicated` _expression (delegate `OnExpressionDuplicated_Event`))
  (`self.Duplicate` _expression))

(event `OnExpressionDuplicated_Event` :!signature `self.OnDuplicated`
  (params (Duplicate :type "/Game/BPSLang/AST/BP_ASTNode Object Reference"))
  ;[1 1 1] Duplicate
  (remove `self.OnDuplicated` (`self.Expression`) (delegate `OnExpressionDuplicated_Event`))
  (bind _returnvalue (`|GenericCreateObject` "BP_ASTNode_UnaryOperation_C" Duplicate (`self.ProgramContext`)))
  (`self.OnDuplicated` _returnvalue))