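; BP_ASTNode_ProgramCall is an expression node in the BPSLang scripting language's AST that calls a named program.
; It executes its Identifier node, looks the resulting name up in the program context's memory, passes its Arguments to that program node and runs it.
; Child results arrive through bound OnExecuted events, and the program's result is copied into a new literal token.
; Failures at any step print a message and report failure.
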(event `self.Execute`
  (params (Origin :type String))
  (bind _identifier (`self.Identifier`))
  ;[1 1 1] Program ID
  (add `self.OnExecuted` _identifier (delegate `OnProgCallIDExec_Event`))
  (`self.Execute` _identifier "Program Call ID"))

(event `OnProgCallIDExec_Event` :!signature `self.OnExecuted`
  (params (Token :type "/Game/BPSLang/Token/BP_SLang_Token Object Reference") (Success :type Boolean))
  (bind (_value _returnvalue) (`BlueprintMapLibrary.Map_Find` (`/Game/BPSLang/AST/BP_ASTNode_Program.Memory` (`self.ProgramContext`)) (`/Game/BPSLang/Token/BP_SLang_Token.Value` Token)))
  ;[1 1 1] Program ID
  (remove `self.OnExecuted` (`self.Identifier`) (delegate `OnProgCallIDExec_Event`))
  (`/Engine/EditorBlueprintResources/StandardMacros.IsValid` Token
    (:`Is Valid`
      (if Success
        ;[1 1 1] Passing args and executing
        (if _returnvalue
          (bind _asbp_astnode_program (cast `/Game/BPSLang/AST/BP_ASTNode_Program` _value)
            (:`then`
              (set `/Game/BPSLang/AST/BP_ASTNode_Program.Arguments` (`self.Arguments`) _asbp_astnode_program)
              (add `self.OnExecuted` _asbp_astnode_program (delegate `OnProgramExecuted_Event`))
              (`self.Execute` _asbp_astnode_program "Program Call"))
            (:`CastFailed`
              (`KismetSystemLibrary.PrintString` null "Node not a program")
              (`self.OnExecuted` null)))
          (else
            (`KismetSystemLibrary.PrintString` null "Program not found in context")
            (`self.OnExecuted` null)))
        (else
          (`KismetSystemLibrary.PrintString` null "Prog Call ID Node invalid or unsuccessful" :!label _label)
          (`self.OnExecuted` null))))
    (:`Is Not Valid`
      (goto _label))))

(event `OnProgramExecuted_Event` :!signature `self.OnExecuted`
  (params (Token :type "/Game/BPSLang/Token/BP_SLang_Token Object Reference") (Success :type Boolean))
  (bind (_value _type) (`/Game/BPSLang/Token/BP_SLang_Token.AsLiteral` Token))
  ;[1 1 1] Passing args and executing
  (remove `self.OnExecuted` (stale `OnProgCallIDExec_Event` _asbp_astnode_program) (delegate `OnProgramExecuted_Event`))
  (`/Engine/EditorBlueprintResources/StandardMacros.IsValid` Token
    (:`Is Valid`
      (if Success
        (bind _returnvalue (`|GenericCreateObject` "/Game/BPSLang/Token/BP_SLang_Token.BP_SLang_Token_C"))
        (`/Game/BPSLang/Token/BP_SLang_Token.MakeLiteral` _returnvalue _value _type)
        (`self.OnExecuted` _returnvalue true)
        (else
          (`KismetSystemLibrary.PrintString` null "Program execution failed or invalid token" :!label _label_2)
          (`self.OnExecuted` null))))
    (:`Is Not Valid`
      (goto _label_2))))