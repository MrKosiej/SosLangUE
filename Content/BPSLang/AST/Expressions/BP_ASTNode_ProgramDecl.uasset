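; AST node Blueprint for a program declaration in the BPSLang scripting language.
; On Execute it constructs a BP_ASTNode_Program with the current ProgramContext and copies that context's OutsideContext onto the new node.
; The declaration appears unfinished: writes to memory, program name and return type, plus the identifier token passed to CallOnExecuted, are disconnected and never run.
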(event `self.Execute`
  (params (Origin :type String))
  (bind _programcontext (`self.ProgramContext`))
  (bind _returnvalue (`|GenericCreateObject` "/Game/BPSLang/AST/BP_ASTNode_Program.BP_ASTNode_Program_C" _programcontext null))
  (set `/Game/BPSLang/AST/BP_ASTNode_Program.OutsideContext` (`/Game/BPSLang/AST/BP_ASTNode_Program.OutsideContext` _programcontext) _returnvalue))