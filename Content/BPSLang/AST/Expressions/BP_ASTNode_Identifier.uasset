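; Identifier expression node in the BPSLang AST, which resolves a variable name to its stored token during interpretation.
; Evaluate looks up the node's Name in the interpreter's ProgramMemory map and returns the found token with success.
; A missing name returns a fallback token with value "0" and failure, and both paths print a debug string tagged with the caller's origin.
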(fn `Evaluate`
  (params (Origin :type String))
  (returns (Token :type "/Game/BPSLang/S_SLangToken Structure") (Success :type Boolean))
  (bind (_value _returnvalue) (`BlueprintMapLibrary.Map_Find` (`/Game/BPSLang/BP_SLangInterpreter.ProgramMemory` (`self.Interpreter`)) (`self.Name`)))
  (bind (_type _value_2) (break `/Game/BPSLang/S_SLangToken` _value))
  (if _returnvalue
    (`KismetSystemLibrary.PrintString` null (`KismetStringLibrary.Concat_StrStr` "Evaluating Identifier from: " Origin " Of Type: " (`|GetEnumeratorNameAsString` _type) " And Value: " _value_2) false)
    (return _value true)
    (else
      (`KismetSystemLibrary.PrintString` null (`KismetStringLibrary.Concat_StrStr` "Evaluating Identifier from: " Origin " | Variable Not Found") false)
      (return (make `/Game/BPSLang/S_SLangToken` "NewEnumerator1") false))))