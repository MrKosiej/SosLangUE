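; AST node for a struct declaration in BPSLang, a scripting language interpreted in Blueprints.
; It evaluates its name node, then uses that identifier as the declared program's name, return type and type.
; That program receives the body's expressions, is executed, and is added by name to the parent context's memory.
; Child results arrive through one-shot OnExecuted bindings, which relay success or failure to the node's caller.
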(event `self.Execute`
  (params (Origin :type String) (ReturnType :type "/Game/BPSLang/E_RefVal Enum" :default "NewEnumerator0"))
  (bind _name (`self.Name`))
  (set `self.ProgramContext` (`/Game/BPSLang/AST/BP_ASTNode.ProgramContext` (`self.DeclaredProgram`)))
  (set `/Game/BPSLang/AST/BP_ASTNode_Program.Expressions` (`/Game/BPSLang/AST/BP_ASTNode_ExpressionsWrapper.Expressions` (`self.Body`)) (`self.DeclaredProgram`))
  ;[1 1 1] Prog Name
  (add `self.OnExecuted` _name (delegate `OnProgNameExecuted_Event`))
  (`self.Execute` _name "Struct Decl Name" "NewEnumerator0"))

(event `OnProgNameExecuted_Event` :!signature `self.OnExecuted`
  (params (Result :type "/Game/BPSLang/AST/BP_ASTNode Object Reference") (Success :type Boolean))
  (bind _value (`self.GetIdentity` Result))
  (bind _programcontext (`self.ProgramContext`))
  (bind _declaredprogram (`self.DeclaredProgram`))
  (bind _declaredprogram_2 (`self.DeclaredProgram`))
  (bind _declaredprogram_3 (`self.DeclaredProgram`))
  (bind _programname (`/Game/BPSLang/AST/BP_ASTNode_Program.ProgramName` (`self.DeclaredProgram`)))
  ;[1 1 1] Prog Name
  (remove `self.OnExecuted` (`self.Name`) (delegate `OnProgNameExecuted_Event`))
  (if Success
    (set `/Game/BPSLang/AST/BP_ASTNode_Program.ProgramName` _value _declaredprogram_3)
    (set `/Game/BPSLang/AST/BP_ASTNode_Program.Return Type` _value _declaredprogram_3)
    (set `/Game/BPSLang/AST/BP_ASTNode.Type` _value _declaredprogram_3)
    (set `/Game/BPSLang/AST/BP_ASTNode_Program.ProgramType` "NewEnumerator1" _declaredprogram_3)
    (add `self.OnExecuted` _declaredprogram_2 (delegate `OnBodyExecuted_Event`))
    (`self.Execute` _declaredprogram_2 "Struct Decl" "NewEnumerator1")
    (`BlueprintMapLibrary.Map_Add` (`/Game/BPSLang/AST/BP_ASTNode_Program.Memory` _programcontext) _programname _declaredprogram)
    (`KismetSystemLibrary.PrintString` null (`KismetStringLibrary.Concat_StrStr` "Saving Program: " _programname " To the memory of " (`/Game/BPSLang/AST/BP_ASTNode_Program.ProgramName` _programcontext) " | dets: " (`/Game/BPSLang/AST/BP_ASTNode_Program.Return Type` _declaredprogram)))
    (else
      (`KismetSystemLibrary.PrintString` null "Struct Name Node invalid or unsuccessful")
      (`self.OnExecuted` null))))

(event `OnBodyExecuted_Event` :!signature `self.OnExecuted`
  (params (Result :type "/Game/BPSLang/AST/BP_ASTNode Object Reference") (Success :type Boolean))
  (remove `self.OnExecuted` (`self.DeclaredProgram`) (delegate `OnBodyExecuted_Event`))
  (if Success
    (`self.OnExecuted` Result true)
    (else
      (`KismetSystemLibrary.PrintString` null "Struct token invalid or unsuccessful")
      (`self.OnExecuted` null))))