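; BP_ASTNode_ExpressionsWrapper is a BPSLang syntax tree node that holds a list of expressions and implements its own duplication.
; Duplication is an event-driven chain: it binds to one expression's OnDuplicated, collects the copy when that fires, unbinds and advances to the next index.
; Once the list is exhausted, it constructs a new wrapper with the same ProgramContext and IdentityToken, assigns the collected copies and broadcasts it through OnDuplicated.
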(event `ContinueDuplication`
  (bind _expressions (`self.Expressions`))
  (bind _duplicationindex (`self.DuplicationIndex`))
  (`/Engine/EditorBlueprintResources/StandardMacros.IncrementInt` (`self.DuplicationIndex`)
    (:`  `
      (if (`KismetArrayLibrary.Array_IsValidIndex` _expressions _duplicationindex) :!label _label
        (add `self.OnDuplicated` (`|GetArrayItem` _expressions _duplicationindex) (delegate `OnDuplicated_Event`))
        (else
          (bind _returnvalue (`|GenericCreateObject` "BP_ASTNode_ExpressionsWrapper_C" (`self.ProgramContext`) (`self.IdentityToken`)))
          (set `/Game/BPSLang/AST/BP_ASTNode_ExpressionsWrapper.Expressions` (`self.ExpressionsDuplicate`) _returnvalue)
          (`self.OnDuplicated` _returnvalue))))))

(event `self.Duplicate`
  (set `self.DuplicationIndex` 0)
  (`KismetArrayLibrary.Array_Clear` (`self.ExpressionsDuplicate`))
  (goto _label))

(event `OnDuplicated_Event` :!signature `self.OnDuplicated`
  (params (Duplicate :type "/Game/BPSLang/AST/BP_ASTNode Object Reference"))
  (remove `self.OnDuplicated` (`|GetArrayItem` (`self.Expressions`) (`self.DuplicationIndex`)) (delegate `OnDuplicated_Event`))
  (`KismetArrayLibrary.Array_Add` (`self.ExpressionsDuplicate`) Duplicate)
  (`self.ContinueDuplication`))