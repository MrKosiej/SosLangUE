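; Base AST node Blueprint for BPSLang, holding an identity made of Value, Type and Domain.
; The identity is set directly through MakeNode or copied from an identity token's standard details by ApplyIdentityToken, and read back through GetIdentity.
; Execute is an empty event taking an origin and return type, while Duplicate only prints a not-implemented warning, leaving both for specific node types to implement.
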(event `Execute`
  (params (Origin :type String) (ReturnType :type "/Game/BPSLang/E_RefVal Enum" :default "NewEnumerator0")))

(event `Duplicate`
  (`KismetSystemLibrary.PrintString` null "Duplicate was not implemented in This Node, please fix first"))

(fn `ApplyIdentityToken`
  (params (IdentityToken :type "/Game/BPSLang/Token/BP_SLang_Token Object Reference"))
  (bind (_value _type _domain) (`/Game/BPSLang/Token/BP_SLang_Token.GetStandardDetails` IdentityToken))
  (set `self.Value` _value)
  (set `self.Type` _type)
  (set `self.Domain` _domain))

(fn `GetIdentity`
  (returns (Value :type String) (Type :type String) (Domain :type "/Game/BPSLang/E_TokenDomain Enum"))
  (return (`self.Value`) (`self.Type`) (`self.Domain`)))

(fn `MakeNode`
  (params (Value :type String) (Type :type String) (Domain :type "/Game/BPSLang/E_TokenDomain Enum" :default "NewEnumerator0"))
  (set `self.Value` Value)
  (set `self.Type` Type)
  (set `self.Domain` Domain))