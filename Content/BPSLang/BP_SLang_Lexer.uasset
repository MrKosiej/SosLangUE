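; Lexer for the Blueprint-built SLang script language, turning Program.Script into BP_SLang_Token objects stored in Program.LexedTokens.
; Tokenize walks a character array through NextCharacter, skipping line comments, whitespace and commas, and classifying characters by ASCII code.
; It emits number and string literals, letter-only keywords, types and identifiers, and operators from lookup databases, trying two-character operators first.
; A float literal with multiple dots aborts lexing and returns false.
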(fn `NextCharacter`
  (returns (Success :type Boolean))
  (bind _scriptcharacters (`self.ScriptCharacters`))
  (bind _result (`/Engine/EditorBlueprintResources/StandardMacros.IncrementInt` (`self.Position`))
    (:`  `
      (if (`KismetArrayLibrary.Array_IsValidIndex` _scriptcharacters _result)
        (set `self.CurrentChar` (`|GetArrayItem` _scriptcharacters _result))
        (return true)
        (else
          (set `self.NextCharFailed` true)
          (return false))))))

(fn `Tokenize`
  (returns (Success :type Boolean))
  (bind _scriptcharacters (`self.ScriptCharacters`))
  (bind _tokenbuilder (`self.TokenBuilder`))
  (bind _tokenbuilder_2 (`self.TokenBuilder`))
  (bind _currentchar (`self.CurrentChar`))
  (bind _scriptcharacters_2 (`self.ScriptCharacters`))
  (bind _position (`self.Position`))
  (bind _currentchar_2 (`self.CurrentChar`))
  (bind _position_2 (`self.Position`))
  (bind _returnvalue (`KismetArrayLibrary.Array_Contains` (`self.Keywords`) (`self.CurrentChar`)))
  (bind _returnvalue_2 (`KismetStringLibrary.EqualEqual_StrStr` (`self.CurrentChar`) "\""))
  (bind _returnvalue_3 (`KismetStringLibrary.GetCharacterAsNumber` (`self.CurrentChar`)))
  (bind _returnvalue_4 (+ (`self.Position`) 1))
  (bind _returnvalue_5 (`KismetArrayLibrary.Array_Contains` (`KismetStringLibrary.GetCharacterArrayFromString` (`self.TokenBuilder`)) "."))
  (bind _returnvalue_6 (`KismetMathLibrary.InRange_IntInt` _returnvalue_3 48 57))
  (bind (_value _returnvalue_7) (`BlueprintMapLibrary.Map_Find` (`/Game/BPSLang/BP_SLang_OperatorsDatabase.Database` (`self.OperatorsData`)) _currentchar))
  (bind _returnvalue_8 (== _returnvalue_3 46))
  (bind _returnvalue_9 (`KismetMathLibrary.InRange_IntInt` (`KismetStringLibrary.GetCharacterAsNumber` (`KismetStringLibrary.ToUpper` (`self.CurrentChar`))) 65 90))
  (bind _returnvalue_10 (`KismetStringLibrary.Concat_StrStr` _currentchar (`|GetArrayItem` _scriptcharacters _returnvalue_4)))
  ;[1 1 1] Break down the script to characters and save Len
  (set `self.NextCharFailed` false)
  (`KismetArrayLibrary.Array_Clear` (`self.Tokens`))
  (bind _output_get (set `self.ScriptCharacters` (`KismetStringLibrary.GetCharacterArrayFromString` (`/Game/BPSLang/AST/BP_ASTNode_Program.Script` (`self.Program`)))))
  (set `self.CurrentChar` (`|GetArrayItem` _output_get _position))
  (bind _returnvalue_11 (and (`KismetArrayLibrary.Array_IsValidIndex` _output_get _position) (not (`self.NextCharFailed`))))
  (while _returnvalue_11
    (set `self.TokenBuilder` "")
    (if (`KismetArrayLibrary.Array_IsValidIndex` _output_get (+ _position 1))
      (if (and (`KismetStringLibrary.EqualEqual_StrStr` (`|GetArrayItem` _scriptcharacters_2 _position_2) "/") (`KismetStringLibrary.EqualEqual_StrStr` (`|GetArrayItem` _scriptcharacters_2 (+ _position_2 1)) "/"))
        (while (and (not (== (`KismetStringLibrary.GetCharacterAsNumber` (`self.CurrentChar`)) 10)) _returnvalue_11)
          (`self.NextCharacter`))
        (else
          ;[1 1 1] Skip White Characters and coma separator
          (if (or (`KismetStringLibrary.EqualEqual_StrStr` _currentchar_2 " ") (`KismetStringLibrary.IsEmpty` _currentchar_2) (== (`KismetStringLibrary.GetCharacterAsNumber` _currentchar_2) 10) (`KismetStringLibrary.EqualEqual_StrStr` _currentchar_2 ",")) :!label _label
            (`self.NextCharacter`)
            (else
              ;[1 1 1] Integer/ Float
              (if _returnvalue_6
                (while (and (or _returnvalue_8 _returnvalue_6) (not (`self.NextCharFailed`)))
                  (if _returnvalue_8
                    (if (not _returnvalue_5)
                      _
                      (else
                        (`KismetSystemLibrary.PrintString` null "Found 2+ dots in float literal")
                        (return false))))
                  (set `self.TokenBuilder` (`KismetStringLibrary.Concat_StrStr` (`self.TokenBuilder`) (`self.CurrentChar`)))
                  (`self.NextCharacter`))
                (bind _returnvalue_12 (`|GenericCreateObject` "/Game/BPSLang/Token/BP_SLang_Token.BP_SLang_Token_C"))
                (`/Game/BPSLang/Token/BP_SLang_Token.MakeLiteral` _returnvalue_12 (`self.TokenBuilder`) (select `bool` _returnvalue_5 :`false` "int" :`true` "float"))
                (`KismetArrayLibrary.Array_Add` (`self.Tokens`) _returnvalue_12)
                (else
                  ;[1 1 1] Strings
                  (if _returnvalue_2
                    (`self.NextCharacter`)
                    (while (and (not _returnvalue_2) (not (`self.NextCharFailed`)))
                      (set `self.TokenBuilder` (`KismetStringLibrary.Concat_StrStr` (`self.TokenBuilder`) (`self.CurrentChar`)))
                      (`self.NextCharacter` :!label _label_2))
                    (`|ExecutionSequence`
                      (:`then_0`
                        (goto _label_2))
                      (:`then_1`
                        (bind _returnvalue_13 (`|GenericCreateObject` "/Game/BPSLang/Token/BP_SLang_Token.BP_SLang_Token_C"))
                        (`/Game/BPSLang/Token/BP_SLang_Token.MakeLiteral` _returnvalue_13 (`self.TokenBuilder`) "string")
                        (`KismetArrayLibrary.Array_Add` (`self.Tokens`) _returnvalue_13)))
                    (else
                      ;[1 1 1] Keyword/ Identifier/ Type
                      (if (or _returnvalue_9 _returnvalue)
                        (if _returnvalue
                          (set `self.TokenBuilder` (`self.CurrentChar`))
                          (`self.NextCharacter`)
                          (else
                            (while (and _returnvalue_9 (not (`self.NextCharFailed`)))
                              (set `self.TokenBuilder` (`KismetStringLibrary.Concat_StrStr` (`self.TokenBuilder`) (`self.CurrentChar`)))
                              (`self.NextCharacter`))))
                        (bind _returnvalue_14 (`|GenericCreateObject` "/Game/BPSLang/Token/BP_SLang_Token.BP_SLang_Token_C"))
                        (if (`KismetArrayLibrary.Array_Contains` (`self.Keywords`) _tokenbuilder)
                          (`/Game/BPSLang/Token/BP_SLang_Token.MakeKeyword` _returnvalue_14 _tokenbuilder_2)
                          (elif (`KismetArrayLibrary.Array_Contains` (`self.StandardTypes`) _tokenbuilder)
                            (`/Game/BPSLang/Token/BP_SLang_Token.MakeType` _returnvalue_14 _tokenbuilder_2)
                            (else
                              (`/Game/BPSLang/Token/BP_SLang_Token.MakeIdentifier` _returnvalue_14 _tokenbuilder_2 ""))))
                        (`KismetArrayLibrary.Array_Add` (`self.Tokens`) _returnvalue_14)
                        (else
                          ;[1 1 1] Operators
                          (if _returnvalue_7
                            (if (`KismetArrayLibrary.Array_IsValidIndex` _scriptcharacters _returnvalue_4)
                              (if (`.ReturnValue` (`BlueprintMapLibrary.Map_Find` (`/Game/BPSLang/BP_SLang_OperatorsDatabase.Database` (`self.DoubleOperatorsData`)) _returnvalue_10)) :!label _label_3
                                (bind _returnvalue_15 (`|GenericCreateObject` "/Game/BPSLang/Token/BP_SLang_Token.BP_SLang_Token_C"))
                                (`/Game/BPSLang/Token/BP_SLang_Token.MakeOperator` _returnvalue_15 _returnvalue_10)
                                (`KismetArrayLibrary.Array_Add` (`self.Tokens`) _returnvalue_15)
                                (`self.NextCharacter`)
                                (else
                                  (if _returnvalue_7 :!label _label_4
                                    (bind _returnvalue_16 (`|GenericCreateObject` "/Game/BPSLang/Token/BP_SLang_Token.BP_SLang_Token_C"))
                                    (`/Game/BPSLang/Token/BP_SLang_Token.MakeOperator` _returnvalue_16 (`self.CurrentChar`))
                                    (`KismetArrayLibrary.Array_Add` (`self.Tokens`) _returnvalue_16))))
                              (else
                                (goto _label_4)))
                            (else
                              (goto _label_3)))
                          (`self.NextCharacter`)))))))))))
      (else
        (goto _label))))
  (set `/Game/BPSLang/AST/BP_ASTNode_Program.LexedTokens` (`self.Tokens`) (`self.Program`))
  (return true))